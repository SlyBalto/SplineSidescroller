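; Projectile bullet that holds a constant speed, hovers at a height above the ground and bends along TurnSpline corners, expiring after LifeSpan or on bounce.
; Tick traces down to keep height and tilt to the slope, re-basing the height on large changes.
; Overlapping a TurnSpline box plane-constrains the bullet to that end's arrow.
; Dot-product and distance tests then switch between snapping along the spline by Direction and releasing it, with debug prints throughout.
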(event `self.ReceiveBeginPlay`
  (bind _lifespan (`self.LifeSpan`))
  (bind _projectilemovement (`self.ProjectileMovement`))
  (bind _returnvalue (`SceneComponent.K2_GetComponentLocation` (`self.BulletMesh`)))
  (bind (_outhit _returnvalue_2) (`KismetSystemLibrary.LineTraceSingleForObjects` _returnvalue (- _returnvalue (0.0 0.0 1500.0)) (`|MakeArray` "ObjectTypeQuery1" :!type "EObjectTypeQuery Enum")))
  (if _returnvalue_2
    (set `self.TargetHeight` (`.Distance` (`GameplayStatics.BreakHitResult` _outhit))))
  (`MovementComponent.SetUpdatedComponent` (`self.ProjectileMovement`) (`self.BulletMesh`))
  (set `MovementComponent.Velocity` (* (`KismetMathLibrary.Normal` (`MovementComponent.Velocity` _projectilemovement)) (`self.TargetSpeed`)) _projectilemovement)
  (if (> _lifespan 0.0)
    (`KismetSystemLibrary.Delay` _lifespan)
    (`self.K2_DestroyActor`)))

(event `SplineAlign`
  (bind _projectilemovement (`self.ProjectileMovement`))
  (bind _bulletmesh (`self.BulletMesh`))
  (bind _splinedistance (`self.SplineDistance`))
  (bind _returnvalue (`|EnumEquality` (`self.Direction`) "NewEnumerator1"))
  (bind _spline (`/Game/Blueprints/SplineStuff/TurnSpline.Spline` (`self.TurnSpline`)))
  (bind _spline_2 (`/Game/Blueprints/SplineStuff/TurnSpline.Spline` (`self.TurnSpline`)))
  (bind _spline_3 (`/Game/Blueprints/SplineStuff/TurnSpline.Spline` (`self.TurnSpline`)))
  (bind _returnvalue_2 (`SplineComponent.GetLocationAtDistanceAlongSpline` _spline_3 _splinedistance "World"))
  (bind _returnvalue_3 (`KismetMathLibrary.MakeVector` (.x _returnvalue_2) (.y _returnvalue_2) (.z (`SceneComponent.K2_GetComponentLocation` _bulletmesh))))
  (bind _returnvalue_4 (+ (* (* (`/Game/Blueprints/Object_MacroLibrary.VectorRemoveZ` (`SplineComponent.FindTangentClosestToWorldLocation` _spline_2 (`SceneComponent.K2_GetComponentLocation` (`self.BulletMesh`)) "World")) 30.0) (select `/Game/Blueprints/Direction` (`self.Direction`) :`NewEnumerator0` -1.0 :`NewEnumerator1` 1.0 :!type "Float (single-precision)")) (`SceneComponent.K2_GetComponentLocation` (`self.BulletMesh`))))
  (bind _returnvalue_5 (* (`KismetMathLibrary.GetForwardVector` (`KismetMathLibrary.FindLookAtRotation` _returnvalue_2 (select `bool` (`self.use find loc closest / WorldLocationCorrection`) :`false` (+ (* (`SplineComponent.GetDirectionAtDistanceAlongSpline` _spline_3 _splinedistance "World") 55.0 (`/Game/Blueprints/Object_MacroLibrary.BoolFloatFlipper` 1.0 _returnvalue)) _returnvalue_2) :`true` (`SplineComponent.GetLocationAtDistanceAlongSpline` (`/Game/Blueprints/SplineStuff/TurnSpline.Spline` (`self.TurnSpline`)) (+ _splinedistance (`/Game/Blueprints/Object_MacroLibrary.BoolFloatFlipper` 55.0 _returnvalue)) "World")))) (`self.TargetSpeed`)))
  (bind (_x _y _z) (`KismetMathLibrary.BreakVector3f` _returnvalue_5))
  (bind (_returnvalue_x _returnvalue_y _returnvalue_z) (`KismetMathLibrary.BreakVector` (`SplineComponent.GetLocationAtDistanceAlongSpline` _spline_3 (`SplineComponent.GetDistanceAlongSplineAtSplineInputKey` _spline_3 (`SplineComponent.FindInputKeyClosestToWorldLocation` _spline_3 _returnvalue_4)) "World")))
  (set `self.ReachedSplineEnd` false)
  (`MovementComponent.SetPlaneConstraintNormal` _projectilemovement (0.0 0.0 0.0))
  (`KismetSystemLibrary.PrintString` (`KismetStringLibrary.Conv_DoubleToString` (`KismetMathLibrary.Vector_Distance` (`SplineComponent.FindLocationClosestToWorldLocation` _spline_2 _returnvalue_4 "World") (`KismetMathLibrary.MakeVector` (.x _returnvalue_4) (.y _returnvalue_4) _returnvalue_z))) true true (struct :`R` 1.0 :`G` 0.771869 :`B` 0.397902 :`A` 1.0) 0.5 "bulletDistance")
  (set `self.SplineDistance` (`SplineComponent.GetDistanceAlongSplineAtSplineInputKey` _spline (`SplineComponent.FindInputKeyClosestToWorldLocation` _spline (`KismetMathLibrary.MakeVector` (.x (`SceneComponent.K2_GetComponentLocation` (`self.BulletMesh`))) (.y (`SceneComponent.K2_GetComponentLocation` (`self.BulletMesh`))) (.z (`SplineComponent.GetLocationAtDistanceAlongSpline` _spline (`self.SplineDistance`) "World"))))))
  (`KismetSystemLibrary.PrintString` (`KismetStringLibrary.Concat_StrStr` "bullet velocitylength :" (`KismetStringLibrary.Conv_DoubleToString` (`KismetMathLibrary.VSize` _returnvalue_5)) " --- bullet loc vs target loc distance = " (`KismetStringLibrary.Conv_DoubleToString` (`KismetMathLibrary.Vector_Distance` (`.JustRemove Z` (`/Game/Blueprints/Object_MacroLibrary.VectorRemoveZ` _returnvalue_3)) (`.JustRemove Z` (`/Game/Blueprints/Object_MacroLibrary.VectorRemoveZ` (`SceneComponent.K2_GetComponentLocation` (`self.BulletMesh`))))))) true true (struct :`R` 0.930721 :`G` 1.0 :`B` 0.100721 :`A` 1.0) 2.0 "bulletangent")
  (if (`self.use find loc closest / WorldLocationCorrection`)
    _
    (else
      _))
  (`SceneComponent.K2_SetWorldLocation` _bulletmesh _returnvalue_3 false true)
  (bind _output_get (set `MovementComponent.Velocity` (`KismetMathLibrary.MakeVector` _x _y _z) _projectilemovement)))

(event `self.ReceiveTick`
  (params (DeltaSeconds :type "Float (single-precision)"))
  (bind _projectilemovement (`self.ProjectileMovement`))
  (bind _bulletmesh (`self.BulletMesh`))
  (bind _returnvalue (`SceneComponent.K2_GetComponentLocation` (`self.BulletMesh`)))
  (bind _velocity (`MovementComponent.Velocity` _projectilemovement))
  (bind (_returnvalue_roll _returnvalue_pitch _returnvalue_yaw) (`KismetMathLibrary.BreakRotator` (`KismetMathLibrary.FindLookAtRotation` (0.0 0.0 0.0) _velocity)))
  (bind (_outhit _returnvalue_2) (`KismetSystemLibrary.LineTraceSingleForObjects` _returnvalue (- _returnvalue (`KismetMathLibrary.MakeVector` 0.0 0.0 (+ (`self.TargetHeight`) 200.0))) (`|MakeArray` "ObjectTypeQuery1" :!type "EObjectTypeQuery Enum")))
  (set `MovementComponent.Velocity` (* (`KismetMathLibrary.Normal` _velocity) (`self.TargetSpeed`)) _projectilemovement)
  (if _returnvalue_2
    (`SceneComponent.K2_SetWorldRotation` (`self.BulletMesh`) (`KismetMathLibrary.MakeRotator` _returnvalue_roll (* (`.OutSlopeRollDegreeAngle` (`KismetMathLibrary.GetSlopeDegreeAngles` (`SceneComponent.GetRightVector` _bulletmesh) (`.ImpactNormal` (`GameplayStatics.BreakHitResult` _outhit)) (`SceneComponent.GetUpVector` _bulletmesh))) -1.0) _returnvalue_yaw) false false)
    (`KismetSystemLibrary.PrintString` (`KismetStringLibrary.Concat_StrStr` "impact normal: " (`KismetStringLibrary.Conv_VectorToString` (`.ImpactNormal` (`GameplayStatics.BreakHitResult` _outhit))) " -- level difference: " (`KismetStringLibrary.Conv_DoubleToString` (- (`self.minHeight`) (`.Distance` (`GameplayStatics.BreakHitResult` _outhit))))) true true (struct :`R` 0.513876 :`G` 1.0 :`B` 0.996685 :`A` 1.0) 2.0 "diffence Bullet")
    (bind _returnvalue_3 (- (`self.TargetHeight`) (`.Distance` (`GameplayStatics.BreakHitResult` _outhit))))
    (if (> (`KismetMathLibrary.Abs` _returnvalue_3) 80.0)
      (set `self.TargetHeight` (`.Distance` (`GameplayStatics.BreakHitResult` _outhit))))
    (`SceneComponent.K2_AddWorldOffset` (`self.BulletMesh`) (`KismetMathLibrary.MakeVector` 0.0 0.0 _returnvalue_3) false true) ; This may be less  performance intensive vs setting\nthe location of the bullet with Set Actor Location
    (else
      (`SceneComponent.K2_SetWorldRotation` (`self.BulletMesh`) (`KismetMathLibrary.FindLookAtRotation` (0.0 0.0 0.0) (`MovementComponent.Velocity` (`self.ProjectileMovement`))) false false)))
  (`self.TurnSpline`
    (:`then`
      (`self.SetToSpline`))
    (:`else`)))

(event `TestIfAtFirstBox`
  (bind _spline (`/Game/Blueprints/SplineStuff/TurnSpline.Spline` (`self.TurnSpline`)))
  (`self.TurnSpline`
    (:`then`
      (set `self.AtFirstBox` (< (`SplineComponent.GetDistanceAlongSplineAtSplineInputKey` _spline (`SplineComponent.FindInputKeyClosestToWorldLocation` _spline (`SceneComponent.K2_GetComponentLocation` (`self.BulletMesh`)))) 300.0)))
    (:`else`)))

(event `SetToSpline`
  (bind _projectilemovement (`self.ProjectileMovement`))
  (bind _turnspline (`self.TurnSpline`))
  (bind _turnspline_2 (`self.TurnSpline`))
  (bind _atfirstbox (`self.AtfirstBox`))
  (bind _turnspline_3 (`self.TurnSpline`))
  (bind _spline (`/Game/Blueprints/SplineStuff/TurnSpline.Spline` (`self.TurnSpline`)))
  (bind _returnvalue (select `bool` (`self.AtFirstBox`) :`false` (`/Game/Blueprints/SplineStuff/TurnSpline.ArrowB` _turnspline) :`true` (`/Game/Blueprints/SplineStuff/TurnSpline.ArrowA` _turnspline)))
  (bind _returnvalue_2 (select `bool` _atfirstbox :`false` (`/Game/Blueprints/SplineStuff/TurnSpline.ArrowB` _turnspline_2) :`true` (`/Game/Blueprints/SplineStuff/TurnSpline.ArrowA` _turnspline_2) :!type "SceneComponent Object Reference"))
  (bind _returnvalue_3 (`KismetMathLibrary.Dot_VectorVector` (`KismetMathLibrary.Normal` (- (`SceneComponent.K2_GetComponentLocation` _returnvalue_2) (`SceneComponent.K2_GetComponentLocation` (`self.BulletMesh`)))) (select `bool` _atfirstbox :`false` (* (`SceneComponent.GetForwardVector` _returnvalue_2) -1.0) :`true` (`SceneComponent.GetForwardVector` _returnvalue_2))))
  (`KismetSystemLibrary.PrintString` (`KismetStringLibrary.Concat_StrStr` (select `bool` (`self.AtFirstBox`) :`false` "at 2nd box" :`true` "at 1st box") (`KismetStringLibrary.Concat_StrStr` " reached spline end: " (`KismetStringLibrary.Conv_BoolToString` (`self.ReachedSplineEnd`)) " --- ") (`KismetStringLibrary.Concat_StrStr` "bullet distance: " (`KismetStringLibrary.Conv_DoubleToString` (`self.SplineDistance`)) " in front of arrow: " (`KismetStringLibrary.Conv_BoolToString` (> _returnvalue_3 0.0)))) true true (struct :`G` 0.66 :`B` 1.0 :`A` 1.0) 2.0 "bullet info")
  (if (`self.ReachedSplineEnd`)
    (if (< _returnvalue_3 0.0)
      (if (`KismetMathLibrary.InRange_FloatFloat` (`SplineComponent.GetDistanceAlongSplineAtSplineInputKey` _spline (`SplineComponent.FindInputKeyClosestToWorldLocation` _spline (`SceneComponent.K2_GetComponentLocation` (`self.BulletMesh`)))) 0.0 (`SplineComponent.GetSplineLength` _spline) false false) :!label _label
        (`self.SplineAlign`)
        (goto _label_2 :!via `Reset`)
        (else
          _)))
    (else
      (`self.TestIfAtFirstBox`)
      (goto _label)))
  (`self.TestIfReachedSplineEnd`)
  (`|ExecutionSequence`
    (:`then_0`
      (`/Engine/EditorBlueprintResources/StandardMacros.DoOnce` false :!label _label_2 ; Had issues where bullets would try aligning far past when it needed to, causing stops and other issues
        (:`Completed`
          (`MovementComponent.SetPlaneConstraintNormal` _projectilemovement (`.JustRemove Z` (`/Game/Blueprints/Object_MacroLibrary.VectorRemoveZ` (`SceneComponent.GetRightVector` _returnvalue))))
          (set `MovementComponent.Velocity` (* (select `bool` (`self.AtFirstBox`) :`false` (`SceneComponent.GetForwardVector` (`/Game/Blueprints/SplineStuff/TurnSpline.ArrowB` _turnspline_3)) :`true` (`SceneComponent.GetForwardVector` (`/Game/Blueprints/SplineStuff/TurnSpline.ArrowA` _turnspline_3))) (`self.TargetSpeed`) (`/Game/Blueprints/Object_MacroLibrary.BoolFloatFlipper` 1.0 (`|EnumEquality` (`self.Direction`) "NewEnumerator1"))) _projectilemovement))))
    (:`then_1`
      (if (> (* (`KismetMathLibrary.Vector_Distance` (`.JustRemove Z` (`/Game/Blueprints/Object_MacroLibrary.VectorRemoveZ` (`SceneComponent.K2_GetComponentLocation` _returnvalue))) (`.JustRemove Z` (`/Game/Blueprints/Object_MacroLibrary.VectorRemoveZ` (`SceneComponent.K2_GetComponentLocation` (`self.BulletMesh`))))) _returnvalue_3) 300.0)
        (set `self.TurnSpline` null)
        (`KismetSystemLibrary.PrintString` "Bullet - Spline Reference Removed" true true (struct :`R` 1.0 :`G` 0.290672 :`B` 0.644788 :`A` 1.0))))))

(event `TestIfReachedSplineEnd`
  (bind _atfirstbox (`self.AtFirstBox`))
  (bind _turnspline (`self.TurnSpline`))
  (bind _turnspline_2 (`self.TurnSpline`))
  (bind _atfirstbox_2 (`self.AtfirstBox`))
  (bind _returnvalue (select `bool` _atfirstbox_2 :`false` (`/Game/Blueprints/SplineStuff/TurnSpline.ArrowB` _turnspline_2) :`true` (`/Game/Blueprints/SplineStuff/TurnSpline.ArrowA` _turnspline_2) :!type "SceneComponent Object Reference"))
  (bind _returnvalue_2 (> (`KismetMathLibrary.Vector_Distance` (`.JustRemove Z` (`/Game/Blueprints/Object_MacroLibrary.VectorRemoveZ` (`SceneComponent.K2_GetComponentLocation` (select `bool` _atfirstbox :`false` (`/Game/Blueprints/SplineStuff/TurnSpline.ArrowB` _turnspline) :`true` (`/Game/Blueprints/SplineStuff/TurnSpline.ArrowA` _turnspline))))) (`.JustRemove Z` (`/Game/Blueprints/Object_MacroLibrary.VectorRemoveZ` (`SceneComponent.K2_GetComponentLocation` (`self.BulletMesh`))))) 50.0))
  (bind _returnvalue_3 (> (`KismetMathLibrary.Dot_VectorVector` (`KismetMathLibrary.Normal` (- (`SceneComponent.K2_GetComponentLocation` _returnvalue) (`SceneComponent.K2_GetComponentLocation` (`self.BulletMesh`)))) (select `bool` _atfirstbox_2 :`false` (* (`SceneComponent.GetForwardVector` _returnvalue) -1.0) :`true` (`SceneComponent.GetForwardVector` _returnvalue))) 0.0))
  (`self.TurnSpline`
    (:`then`
      (bind _output_get (set `self.ReachedSplineEnd` (or (and _atfirstbox _returnvalue_2 _returnvalue_3) (and (not _atfirstbox) _returnvalue_2 _returnvalue_3)))))
    (:`else`)))

(event `self.BulletMesh.OnComponentBeginOverlap`
  (params (OverlappedComponent :type "PrimitiveComponent Object Reference") (OtherActor :type "Actor Object Reference") (OtherComp :type "PrimitiveComponent Object Reference") (OtherBodyIndex :type Integer) (bFromSweep :type Boolean) (SweepResult :type "HitResult Structure (by ref)"))
  (bind _atfirstbox (`self.AtFirstBox`))
  (bind _returnvalue (not (`self.AtFirstBox`)))
  (bind _asturn_spline (cast `/Game/Blueprints/SplineStuff/TurnSpline` OtherActor))
  (if (== OtherComp (`/Game/Blueprints/SplineStuff/TurnSpline.BoxA` _asturn_spline))
    ;[1 1 1] overlapped with left Box for Spline
    (set `self.ReachedSplineEnd` false)
    (`MovementComponent.SetPlaneConstraintNormal` (`self.ProjectileMovement`) (`SceneComponent.GetRightVector` (`/Game/Blueprints/SplineStuff/TurnSpline.ArrowA` _asturn_spline)))
    (bind _turnspline (`self.TurnSpline`)
      (:`then`
        (if (or (!= _turnspline _asturn_spline) _returnvalue)
          (`KismetSystemLibrary.PrintString` (select `bool` _returnvalue :`true` "reseting, thinks still at 2nd box"))
          (set `self.SplineDistance` 0.0 :!label _label_3)
          (set `self.TurnSpline` _asturn_spline)))
      (:`else`
        (goto _label_3)))
    (elif (== OtherComp (`/Game/Blueprints/SplineStuff/TurnSpline.BoxB` _asturn_spline))
      ;[1 0.5487 0.6634] overlap with right spline box
      (set `self.ReachedSplineEnd` false)
      (`MovementComponent.SetPlaneConstraintNormal` (`self.ProjectileMovement`) (`SceneComponent.GetRightVector` (`/Game/Blueprints/SplineStuff/TurnSpline.ArrowB` _asturn_spline)))
      (bind _turnspline_2 (`self.TurnSpline`)
        (:`then`
          (if (or _atfirstbox (!= _turnspline_2 _asturn_spline))
            (`KismetSystemLibrary.PrintString` (select `bool` _atfirstbox :`true` "reseting, thinks still at first box"))
            (set `self.SplineDistance` (`SplineComponent.GetSplineLength` (`/Game/Blueprints/SplineStuff/TurnSpline.Spline` _asturn_spline)) :!label _label_4)
            (set `self.TurnSpline` _asturn_spline)))
        (:`else`
          (goto _label_4))))))

(event `self.ProjectileMovement.OnProjectileBounce`
  (params (ImpactResult :type "HitResult Structure (by ref)") (ImpactVelocity :type "Vector Structure (by ref)"))
  (`self.K2_DestroyActor`))

(fn `UserConstructionScript`)