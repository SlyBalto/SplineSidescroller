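; Side-on follow camera actor attached to the player character, with yaw that either follows the player or holds a set angle.
; Each tick it eases spring arm yaw and camera side offset toward the facing direction, and tilts the camera down during fast falls unless a custom arm pitch is set.
; Events set arm length, facing and yaw inheritance; the alternate-camera blend is disconnected.
; Rotation lag starts one second after BeginPlay.
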(event `SetTargetPitch`
  (bind _returnvalue (`self.GetVelocity` (`self.GetAttachParentActor`)))
  (`KismetSystemLibrary.PrintString` (`KismetStringLibrary.Conv_VectorToString` _returnvalue) true true (struct :`R` 0.082136 :`G` 0.34375 :`B` 0.211086 :`A` 1.0) 2.0 "targetspeed")
  (set `self.TargetPitch` (select `bool` (!= (`self.CustomSpringArmPitch`) 0.0) :`false` (`KismetMathLibrary.FInterpTo` (`self.TargetPitch`) (`KismetMathLibrary.MapRangeClamped` (`.Z` (`KismetMathLibrary.BreakVector3f` _returnvalue)) -3000.0 -1300.0 -20.0) (`GameplayStatics.GetWorldDeltaSeconds`) 8.0) :!type "Float (single-precision)")))

(event `self.ReceiveTick`
  (params (DeltaSeconds :type "Float (single-precision)"))
  (bind _returnvalue (`self.GetAttachParentActor`))
  (bind _springarm (`self.SpringArm`))
  (bind _returnvalue_2 (`KismetMathLibrary.Conv_BoolToDouble` (`self.UsePlayerRotation`)))
  (bind (_returnvalue_roll _returnvalue_pitch _returnvalue_yaw) (`KismetMathLibrary.BreakRotator` (`self.K2_GetActorRotation` _returnvalue)))
  (bind (_relativerotation_roll _relativerotation_pitch _relativerotation_yaw) (`KismetMathLibrary.BreakRotator` (`SceneComponent.RelativeRotation` _springarm)))
  (bind (_relativelocation_x _relativelocation_y) (`KismetMathLibrary.BreakVector` (`SceneComponent.RelativeLocation` (`self.Camera`))))
  (if (`self.UsePlayerRotation`)
    (set `self.TargetCameraZRotation` _returnvalue_yaw))
  (set `self.PlayerVsTargetCamZAlpha` (`KismetMathLibrary.FInterpTo` (`self.PlayerVsTargetCamZAlpha`) _returnvalue_2 (`GameplayStatics.GetWorldDeltaSeconds`) 3.0))
  (`self.K2_SetActorRotation` (`KismetMathLibrary.MakeRotator` 0.0 0.0 (.yaw (`KismetMathLibrary.RLerp` (`KismetMathLibrary.MakeRotator` 0.0 0.0 (`self.TargetCameraZRotation`)) (`self.K2_GetActorRotation` _returnvalue) _returnvalue_2 true))))
  (`self.SetTargetPitch`)
  (`SceneComponent.K2_SetRelativeRotation` _springarm (`KismetMathLibrary.MakeRotator` _relativerotation_roll (select `bool` (== (`self.CustomSpringArmPitch`) 0.0) :`false` (`self.CustomSpringArmPitch`) :`true` -7.0 :!type "Float (single-precision)") (`KismetMathLibrary.FInterpTo` _relativerotation_yaw (`self.TargetRelativeRotationZ`) (`GameplayStatics.GetWorldDeltaSeconds`) 5.0)) false false)
  (`SceneComponent.K2_SetRelativeTransform` (`self.Camera`) (`KismetMathLibrary.MakeTransform` (`KismetMathLibrary.MakeVector` 0.0 (`KismetMathLibrary.FInterpTo` _relativelocation_y (`self.TargetCamXOffset`) (`GameplayStatics.GetWorldDeltaSeconds`) 4.0)) (`KismetMathLibrary.MakeRotator` 0.0 (`self.TargetPitch`))) false false))

(event `UseAltCam`
  (params (AltCam :type Boolean))
  (`ActorComponent.SetActive` (`self.Camera`) (not AltCam) false)
  (`ActorComponent.SetActive` (`self.CameraALT`) AltCam false))

(event `UpdateCamera`
  (params (CamTarget :type "/Game/Blueprints/CameraAlt Object Reference"))
  (set `self.CamTarget` CamTarget))

(event `UpdateCamAlt`)

(event `self.ReceiveBeginPlay`
  (bind (_returnvalue_roll _returnvalue_pitch _returnvalue_yaw) (`KismetMathLibrary.BreakRotator` (`self.K2_GetActorRotation` (cast `/Game/Blueprints/Player/BP_ThirdPersonCharacter` (`self.GetAttachParentActor`) :!pure true))))
  (`SceneComponent.SetAbsolute` (`self.Arrow2`) false true false)
  (set `self.TargetCameraZRotation` _returnvalue_yaw)
  (`|ExecutionSequence`
    (:`then_0`
      (`self.UpdateCameraCharFacingOffset` "NewEnumerator1")
      (set `self.TargetTrans` (`SceneComponent.K2_GetComponentToWorld` (`self.Camera`))))
    (:`then_1`
      (`KismetSystemLibrary.Delay` 1.0)
      (set `SpringArmComponent.bEnableCameraRotationLag` true (`self.SpringArm`)))))

(event `UpdateCameraCharFacingOffset`
  (params (SetRotDir :type "/Game/Blueprints/Direction Enum" :default "NewEnumerator0"))
  ;[1 1 1] Camera will use offsets if character is facing left or right
  (bind _output_get (set `self.SetRotDir` SetRotDir))
  (set `self.TargetRelativeRotationZ` (* (+ (select `/Game/Blueprints/Direction` _output_get :`NewEnumerator0` 10.0 :`NewEnumerator1` (* 10.0 -1.0) :!type "Float (single-precision)") 90.0) -1.0))
  (set `self.TargetCamXOffset` (select `/Game/Blueprints/Direction` _output_get :`NewEnumerator0` (* 150.0 -1.0) :`NewEnumerator1` 150.0 :!type "Float (single-precision)")))

(event `ToggleInheritYaw`
  (params (`Inherit Yaw` :type Boolean) (TargetYawIfNotInheriting :type "Float (double-precision)"))
  (set `self.TargetCameraZRotation` TargetYawIfNotInheriting)
  (set `self.UsePlayerRotation` `Inherit Yaw`))

(event `UpdateLength`
  (params (`Target Arm Length` :type "Float (single-precision)" :default 1300.0))
  (set `SpringArmComponent.TargetArmLength` `Target Arm Length` (`self.SpringArm`)))

(fn `UserConstructionScript`
  (bind _returnvalue (`self.GetAttachParentActor`))
  (bind (_returnvalue_roll _returnvalue_pitch _returnvalue_yaw) (`KismetMathLibrary.BreakRotator` (`self.K2_GetActorRotation` _returnvalue)))
  (if (not (`self.Static`))
    (`SceneComponent.SetAbsolute` (`self.Arrow2`) false true false)
    (`self.K2_SetActorRotation` (`KismetMathLibrary.MakeRotator` 0.0 0.0 (+ _returnvalue_yaw 180.0)))
    (`KismetSystemLibrary.PrintString` (`KismetSystemLibrary.GetDisplayName` _returnvalue))))