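; Junction actor that lets a spline-bound third-person character switch between SplineA and SplineB by moving north or south, relative to its right vector.
; Capsule overlap shows direction cones; UpdateRot1 aligns them to the opposite spline's tangent, hiding and disallowing a direction that dead-ends near that spline's ends.
; PlayerSwitch checks that permission, passes a direction dot product and clamped target distance to the character, then refreshes the arrows behind a short re-entry lockout.
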(event `UpdateDirectionChoiceRotation`
  (params (NewRotation :type "Rotator Structure"))
  (`SceneComponent.K2_SetWorldRotation` (`self.NorthArrow`) NewRotation false false))

(event `PlayerSwitch`
  (params (Character :type "/Game/Blueprints/Player/BP_ThirdPersonCharacter Object Reference") (GoingNorth :type Boolean))
  (bind _returnvalue (`self.K2_GetActorLocation` Character))
  (bind _splinea (`self.SplineA`))
  (bind _returnvalue_2 (select `bool` GoingNorth :`false` (`self.GetActorRightVector` Character) :`true` (* (`self.GetActorRightVector` Character) -1.0)))
  (bind _spline (`/Game/Blueprints/SplineStuff/TurnSpline.Spline` (`.CurrentSpline_9_ADBB94374E7CEDCE5F0EFBBE750C5B05` (break `/Game/Blueprints/Mechanics/SplineInfo` (`/Game/Blueprints/Player/BP_ThirdPersonCharacter.SplineInfo` Character)))))
  (bind _normalized (`/Game/Blueprints/Object_MacroLibrary.VectorRemoveZ` (`SplineComponent.GetDirectionAtSplineInputKey` _spline (`SplineComponent.FindInputKeyClosestToWorldLocation` _spline (`self.K2_GetActorLocation` Character)) "World")))
  (if (select `bool` GoingNorth :`false` (`self.AllowSouth`) :`true` (`self.AllowNorth`))
    (`/Engine/EditorBlueprintResources/StandardMacros.DoOnce` false :!label _label
      (:`Completed`
        (`|ExecutionSequence`
          (:`then_0`
            (`/Game/Blueprints/Player/BP_ThirdPersonCharacter.UpdateCurrentSpline` Character (select `bool` (== (`.CurrentSpline_9_ADBB94374E7CEDCE5F0EFBBE750C5B05` (break `/Game/Blueprints/Mechanics/SplineInfo` (`/Game/Blueprints/Player/BP_ThirdPersonCharacter.SplineInfo` Character))) _splinea) :`false` _splinea :`true` (`self.SplineB`)))
            (`KismetSystemLibrary.PrintString` (`KismetStringLibrary.Concat_StrStr` "Character north/south vs Spline Dot Prod: ") true true (struct :`G` 0.0825 :`B` 0.125 :`A` 1.0) 9.0 "switchproduct")
            (`KismetSystemLibrary.DrawDebugArrow` _returnvalue (+ _returnvalue (* _returnvalue_2 100.0)) 20.0 (struct :`R` 1.0 :`B` 0.667171 :`A` 1.0) 5.0 3.0)
            (`KismetSystemLibrary.DrawDebugArrow` _returnvalue (+ (* _normalized 100.0) _returnvalue) 20.0 (struct :`G` 1.0 :`B` 0.729239 :`A` 1.0) 5.0 3.0)
            (`/Game/Blueprints/Player/BP_ThirdPersonCharacter.SwitchToNewSpline` Character (`KismetMathLibrary.Dot_VectorVector` _returnvalue_2 _normalized) true (`KismetMathLibrary.FClamp` (`self.DistanceOnTargetSpline`) 5.0 (- (`SplineComponent.GetSplineLength` (`/Game/Blueprints/SplineStuff/TurnSpline.Spline` (`.CurrentSpline_9_ADBB94374E7CEDCE5F0EFBBE750C5B05` (break `/Game/Blueprints/Mechanics/SplineInfo` (`/Game/Blueprints/Player/BP_ThirdPersonCharacter.SplineInfo` Character))))) 5.0)))
            (`self.UpdateRot1`))
          (:`then_1`
            (`KismetSystemLibrary.Delay` 0.2)
            (goto _label :!via `Reset`)))))))

(event `SetArrowVis`
  (params (Visible :type Boolean))
  (`SceneComponent.SetHiddenInGame` (`self.SouthCone`) (not Visible) false)
  (`SceneComponent.SetHiddenInGame` (`self.NorthCone`) (not Visible) false))

(event `self.Capsule.OnComponentBeginOverlap`
  (params (OverlappedComponent :type "PrimitiveComponent Object Reference") (OtherActor :type "Actor Object Reference") (OtherComp :type "PrimitiveComponent Object Reference") (OtherBodyIndex :type Integer) (bFromSweep :type Boolean) (SweepResult :type "HitResult Structure (by ref)"))
  (bind _asbp_third_person_character (cast `/Game/Blueprints/Player/BP_ThirdPersonCharacter` OtherActor))
  (set `self.Player` _asbp_third_person_character)
  (`self.UpdateRot1`)
  (`self.SetArrowVis` true))

(event `self.Capsule.OnComponentEndOverlap`
  (params (OverlappedComponent :type "PrimitiveComponent Object Reference") (OtherActor :type "Actor Object Reference") (OtherComp :type "PrimitiveComponent Object Reference") (OtherBodyIndex :type Integer))
  (cast `/Game/Blueprints/Player/BP_ThirdPersonCharacter` OtherActor)
  (`self.SetArrowVis` false))

(event `UpdateRot1`
  (bind _splinea (`self.SplineA`))
  (bind _returnvalue (`SceneComponent.K2_GetComponentLocation` (`self.Capsule`)))
  (bind _returnvalue_2 (`SceneComponent.GetForwardVector` (`self.NorthArrow`)))
  (bind _returnvalue_3 (+ (`self.K2_GetActorLocation`) (0.0 0.0 200.0)))
  (bind _spline (`/Game/Blueprints/SplineStuff/TurnSpline.Spline` (select `bool` (== (`.CurrentSpline_9_ADBB94374E7CEDCE5F0EFBBE750C5B05` (break `/Game/Blueprints/Mechanics/SplineInfo` (`/Game/Blueprints/Player/BP_ThirdPersonCharacter.SplineInfo` (`self.Player`)))) _splinea) :`false` _splinea :`true` (`self.SplineB`))))
  (bind _returnvalue_4 (`SplineComponent.FindLocationClosestToWorldLocation` _spline (`SceneComponent.K2_GetComponentLocation` (`self.NorthArrow`)) "World"))
  (bind _returnvalue_5 (`KismetMathLibrary.Dot_VectorVector` (`SceneComponent.GetForwardVector` (`self.NorthArrow`)) (`/Game/Blueprints/Object_MacroLibrary.VectorRemoveZ` (`SplineComponent.FindTangentClosestToWorldLocation` _spline (`self.K2_GetActorLocation` (`self.Player`)) "World"))))
  (bind _returnvalue_6 (< (`KismetMathLibrary.Vector_Distance` (`SplineComponent.GetLocationAtDistanceAlongSpline` _spline 0.0 "World") _returnvalue_4) 150.0))
  (bind _returnvalue_7 (select `bool` _returnvalue_6 :`false` (< _returnvalue_5 0.0) :`true` (> _returnvalue_5 0.0)))
  (bind _returnvalue_8 (select `bool` _returnvalue_7 :`false` _returnvalue_2 :`true` (* _returnvalue_2 -1.0)))
  (`self.Player`
    (:`then`
      (set `self.DistanceOnTargetSpline` (`SplineComponent.GetDistanceAlongSplineAtSplineInputKey` _spline (`SplineComponent.FindInputKeyClosestToWorldLocation` _spline _returnvalue)))
      (`SceneComponent.K2_SetWorldRotation` (`self.NorthArrow`) (`KismetMathLibrary.FindLookAtRotation` (0.0 0.0 0.0) (`/Game/Blueprints/Object_MacroLibrary.VectorRemoveZ` (`SplineComponent.FindTangentClosestToWorldLocation` _spline _returnvalue "World"))) false false)
      (if (or _returnvalue_6 (< (`KismetMathLibrary.Vector_Distance` (`SplineComponent.GetLocationAtDistanceAlongSpline` _spline (`SplineComponent.GetSplineLength` _spline) "World") _returnvalue_4) 150.0))
        (bind _player (`self.Player`)
          (:`then`
            (`SceneComponent.SetVisibility` (select `bool` _returnvalue_7 :`false` (`self.NorthCone`) :`true` (`self.SouthCone`) :!type "SceneComponent Object Reference") false false) ; Set Cone invisible if that direction is dead end
            (`KismetSystemLibrary.DrawDebugArrow` _returnvalue_3 (+ _returnvalue_3 (* _returnvalue_8 100.0)) 5.0 (struct :`R` 1.0 :`G` 0.107261 :`B` 0.277492 :`A` 1.0) 3.0 4.0)
            (if (> (`KismetMathLibrary.Dot_VectorVector` (* (`self.GetActorRightVector` (`self.Player`)) -1.0) _returnvalue_8) 0.0)
              (set `self.AllowNorth` false)
              (else
                (set `self.AllowSouth` false))))
          (:`else`))
        (else
          (`SceneComponent.SetVisibility` (`self.NorthCone`) true false)
          (`SceneComponent.SetVisibility` (`self.SouthCone`) true false)
          (set `self.AllowNorth` true)
          (set `self.AllowSouth` true))))
    (:`else`)))

(fn `UserConstructionScript`
  (`SceneComponent.K2_SetRelativeLocation` (`self.Capsule`) (`KismetMathLibrary.MakeVector` 0.0 0.0 (- (`CapsuleComponent.CapsuleHalfHeight` (`self.Capsule`)) 50.0)) false false))