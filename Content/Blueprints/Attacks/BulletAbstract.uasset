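; BulletAbstract is a base projectile Blueprint for attack bullets, with events intended to be overridden by child bullet types.
; On BeginPlay, SetInitialVelocity launches the ProjectileMovement component along local X at TargetSpeed, then StartLifespan begins a timed removal.
; A positive LifeSpan triggers a delay followed by RemoveBulletFromGame, which destroys the actor.
; An unconnected node chain that would renormalize velocity to TargetSpeed never runs.
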(event `RemoveBulletFromGame`
  ;[1 1 1] These events can be overridden in child blueprints if we need to do something different. for example, setting initial velocity may be different for various kinds of bullets.
  (`self.K2_DestroyActor`))

(event `SetInitialVelocity`
  ;[1 1 1] These events can be overridden in child blueprints if we need to do something different. for example, setting initial velocity may be different for various kinds of bullets.
  (`ProjectileMovementComponent.SetVelocityInLocalSpace` (`self.ProjectileMovement`) (`KismetMathLibrary.MakeVector` (`self.TargetSpeed`))))

(event `self.ReceiveBeginPlay`
  (`self.SetInitialVelocity`)
  (`self.StartLifespan`))

(event `StartLifespan`
  (bind _lifespan (`self.LifeSpan`))
  ;[1 1 1] These events can be overridden in child blueprints if we need to do something different. for example, setting initial velocity may be different for various kinds of bullets.
  (if (> _lifespan 0.0)
    (`KismetSystemLibrary.Delay` _lifespan)
    (`self.RemoveBulletFromGame`)))

(fn `UserConstructionScript`)