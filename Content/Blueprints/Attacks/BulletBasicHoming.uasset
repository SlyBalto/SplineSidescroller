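; BulletBasicHoming is a homing bullet, derived from an abstract bullet, that explodes instead of dealing direct damage.
; BeginPlay skips the parent's, assigning the homing target, launching along local X at TargetSpeed (also the max speed) and starting the lifespan timer.
; Successful damage overlaps, bounces and lifespan expiry all call the overridden RemoveBulletFromGame, which spawns Explosion_Enemy with sender and strength before destroying the bullet.
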(event `self.StartLifespan`
  (bind _lifespan (`self.LifeSpan`))
  (if (> _lifespan 0.0)
    (`KismetSystemLibrary.Delay` _lifespan)
    (`self.RemoveBulletFromGame`)))

(event `Explode`
  (`|SpawnActorFromClass` "/Game/Blueprints/Attacks/Explosion_Enemy.Explosion_Enemy_C" (`KismetMathLibrary.MakeTransform` (`self.K2_GetActorLocation`)) "Undefined" "MultiplyWithRoot" null (`self.SentFrom`) (`self.ExplosionStrength`) null))

(event `self.ReceiveBeginPlay`
  (bind _projectilemovement (`self.ProjectileMovement`))
  (bind _targetspeed (`self.TargetSpeed`))
  ;[1 1 1] This blueprint does not call the Abstract Bullet's Event BeginPlay, meaning it also does not call the Set initial Velocity and Start lifespan.
  (set `ProjectileMovementComponent.HomingTargetComponent` (`self.HomingTargetComp`) (`self.ProjectileMovement`))
  (`ProjectileMovementComponent.SetVelocityInLocalSpace` _projectilemovement (`KismetMathLibrary.MakeVector` _targetspeed))
  (set `ProjectileMovementComponent.MaxSpeed` _targetspeed _projectilemovement)
  (`self.StartLifespan`) ; Normally included in the Abstract parent class's Begin Play, \nbut we're not calling that in this bullet class, so we need to\ncall this event in this blueprint.
)

(event `self.ProjectileMovement.OnProjectileBounce`
  (params (ImpactResult :type "HitResult Structure (by ref)") (ImpactVelocity :type "Vector Structure (by ref)"))
  (`self.RemoveBulletFromGame`))

(event `/Game/Blueprints/Mechanics/HealthAndDamageInterface.DamageSuccessful`
  ;[1 1 1] This bullet does not cause damage when it overlaps with other actors like a player, etc., but it's explosion causes the damage instead. The explosion is activated by either overlapping (causing "damage") or hitting a surface like the floor or a wall. The explosion is included in an overridden version of the Remove Bullet From Game event.
  (`self.RemoveBulletFromGame`))

(event `self.RemoveBulletFromGame`
  ;[1 0.4245 0.1299] New overridden version of the remove bullet from game including the explosion.
  (`self.Explode`)
  (`self.K2_DestroyActor`))

(fn `UserConstructionScript`)