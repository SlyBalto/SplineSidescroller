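; Base-style bullet projectile that follows TurnSpline actors around bends and hugs the ground at a set height.
; Overlapping a spline's end boxes latches it on; each tick it advances along the spline, steering velocity by look-ahead.
; Leaving past an end arrow, it takes that arrow's direction with a plane constraint, then drops the spline reference.
; A downward trace keeps height and pitches the mesh to the surface; bouncing removes it.
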(event `self.ReceiveBeginPlay`
  (bind _turnspline (`self.TurnSpline`))
  (bind (_returnvalue_x _returnvalue_y _returnvalue_z) (`KismetMathLibrary.BreakVector` (`SceneComponent.K2_GetComponentLocation` (`self.BulletMesh`))))
  (bind _returnvalue (`SceneComponent.K2_GetComponentLocation` (`self.BulletMesh`)))
  (`parent.ReceiveBeginPlay`)
  (`/Engine/EditorBlueprintResources/StandardMacros.IsValid` _turnspline
    (:`Is Valid`
      (if (< (`self.GetDotProduct`) 0.0)
        (`SceneComponent.K2_SetWorldLocation` (`self.BulletMesh`) (`KismetMathLibrary.MakeVector` (.x (`SplineComponent.GetLocationAtDistanceAlongSpline` (`/Game/Blueprints/SplineStuff/TurnSpline.Spline` _turnspline) (`self.SplineDistance`) "World")) (.y (`SplineComponent.GetLocationAtDistanceAlongSpline` (`/Game/Blueprints/SplineStuff/TurnSpline.Spline` _turnspline) (`self.SplineDistance`) "World")) _returnvalue_z) false true)))
    (:`Is Not Valid`
      _))
  (bind (_outhit _returnvalue_2) (`KismetSystemLibrary.LineTraceSingleForObjects` _returnvalue (- _returnvalue (0.0 0.0 1400.0)) (`|MakeArray` "ObjectTypeQuery1" :!type "EObjectTypeQuery Enum")))
  (if _returnvalue_2
    (set `self.TargetHeight` (`.Distance` (`GameplayStatics.BreakHitResult` _outhit)))))

(event `SetVelocityOnSpline`
  (params (Velocity :type "Vector Structure"))
  (set `MovementComponent.Velocity` Velocity (`self.ProjectileMovement`)))

(event `SplineAlign`
  (bind _bulletmesh (`self.BulletMesh`))
  (bind _returnvalue (`SplineComponent.GetLocationAtDistanceAlongSpline` (`/Game/Blueprints/SplineStuff/TurnSpline.Spline` (`self.TurnSpline`)) (`self.SplineDistance`) "World"))
  (bind _returnvalue_2 (`SplineComponent.GetSplineLength` (`/Game/Blueprints/SplineStuff/TurnSpline.Spline` (`self.TurnSpline`))))
  (bind _returnvalue_3 (`KismetMathLibrary.FindLookAtRotation` _returnvalue (`SplineComponent.GetLocationAtDistanceAlongSpline` (`/Game/Blueprints/SplineStuff/TurnSpline.Spline` (`self.TurnSpline`)) (`KismetMathLibrary.FClamp` (+ (`KismetMathLibrary.FClamp` (`self.SplineDistance`) 3.0 (- _returnvalue_2 4.0)) (`/Game/Blueprints/Object_MacroLibrary.BoolFloatFlipper` 55.0 (`|EnumEquality` (`self.Direction`) "NewEnumerator1"))) 0.0 _returnvalue_2) "World")))
  (set `self.ReachedSplineEnd` false)
  (`MovementComponent.SetPlaneConstraintNormal` (`self.ProjectileMovement`) (0.0 0.0 0.0))
  (set `self.SplineDistance` (`KismetMathLibrary.FClamp` (+ (`self.SplineDistance`) (* (`self.TargetSpeed`) (`GameplayStatics.GetWorldDeltaSeconds`) (`/Game/Blueprints/Object_MacroLibrary.BoolFloatFlipper` 1.0 (`|EnumEquality` (`self.Direction`) "NewEnumerator1")))) 1.0 (+ (`SplineComponent.GetSplineLength` (`/Game/Blueprints/SplineStuff/TurnSpline.Spline` (`self.TurnSpline`))) -1.0)))
  (`SceneComponent.K2_SetWorldLocation` _bulletmesh (`KismetMathLibrary.MakeVector` (.x _returnvalue) (.y _returnvalue) (.z (`SceneComponent.K2_GetComponentLocation` _bulletmesh))) false true)
  (`self.SetVelocityonSpline` (`KismetMathLibrary.SelectVector` (`MovementComponent.Velocity` (`self.ProjectileMovement`)) (* (`KismetMathLibrary.GetForwardVector` _returnvalue_3) (`self.TargetSpeed`)) (== _returnvalue_3 (struct) :`ErrorTolerance` 0.01))))

(event `SetBulletZLocationTrace`
  (bind _returnvalue (`SceneComponent.K2_GetComponentLocation` (`self.BulletMesh`)))
  (bind (_returnvalue_roll _returnvalue_pitch _returnvalue_yaw) (`KismetMathLibrary.BreakRotator` (`KismetMathLibrary.FindLookAtRotation` (0.0 0.0 0.0) (`MovementComponent.Velocity` (`self.ProjectileMovement`)))))
  (bind (_outhit _returnvalue_2) (`KismetSystemLibrary.LineTraceSingleForObjects` :`Start` _returnvalue :`End` (- _returnvalue (* (0.0 0.0 1.0) 1.0 (+ (`self.TargetHeight`) 200.0))) :`ObjectTypes` (`|MakeArray` "ObjectTypeQuery1" :!type "EObjectTypeQuery Enum") :`bTraceComplex` true :`DrawTime` 1.0))
  (if _returnvalue_2
    (`SceneComponent.K2_SetWorldRotation` (`self.BulletMesh`) (`KismetMathLibrary.MakeRotator` _returnvalue_roll (.pitch (`KismetMathLibrary.Conv_VectorToRotator` (+ (`KismetMathLibrary.RotateAngleAxis` (`.ImpactNormal` (`GameplayStatics.BreakHitResult` _outhit)) 90.0 (`KismetMathLibrary.GreaterGreater_VectorRotator` (`KismetMathLibrary.Normal` (`MovementComponent.Velocity` (`self.ProjectileMovement`))) (struct :`Yaw` 90.0))) (`KismetMathLibrary.Conv_RotatorToVector` (`SceneComponent.K2_GetComponentRotation` (`self.BulletMesh`)))))) _returnvalue_yaw) false false)
    (bind _returnvalue_3 (- (`self.TargetHeight`) (`.Distance` (`GameplayStatics.BreakHitResult` _outhit))))
    (if (> (`KismetMathLibrary.Abs` _returnvalue_3) 80.0)
      (bind _output_get (set `self.TargetHeight` (`.Distance` (`GameplayStatics.BreakHitResult` _outhit))))
      (`KismetSystemLibrary.PrintString` (`KismetStringLibrary.Concat_StrStr` "new height: " (`KismetStringLibrary.Conv_DoubleToString` _output_get))))
    (`SceneComponent.K2_AddWorldOffset` (`self.BulletMesh`) (`KismetMathLibrary.MakeVector` 0.0 0.0 _returnvalue_3) false true) ; This may be less  performance intensive vs setting\nthe location of the bullet with Set Actor Location
    (else
      (`self.SetBulletRotationByVelocity`))))

(event `TestIfAtFirstBox`
  (bind _spline (`/Game/Blueprints/SplineStuff/TurnSpline.Spline` (`self.TurnSpline`)))
  (`self.TurnSpline`
    (:`then`
      (set `self.AtFirstBox` (< (`SplineComponent.GetDistanceAlongSplineAtSplineInputKey` _spline (`SplineComponent.FindInputKeyClosestToWorldLocation` _spline (`SceneComponent.K2_GetComponentLocation` (`self.BulletMesh`)))) 300.0)))
    (:`else`)))

(event `SetToSpline`
  (bind _dotproduct (`self.GetDotProduct`))
  (bind _turnspline (`self.TurnSpline`))
  (bind _spline (`/Game/Blueprints/SplineStuff/TurnSpline.Spline` (`self.TurnSpline`)))
  (bind _returnvalue (select `bool` (`self.AtFirstBox`) :`false` (`/Game/Blueprints/SplineStuff/TurnSpline.ArrowB` _turnspline) :`true` (`/Game/Blueprints/SplineStuff/TurnSpline.ArrowA` _turnspline)))
  (`KismetSystemLibrary.PrintString` (`KismetStringLibrary.Concat_StrStr` (select `bool` (`self.AtFirstBox`) :`false` "at 2nd box" :`true` "at 1st box") (`KismetStringLibrary.Concat_StrStr` " reached spline end: " (`KismetStringLibrary.Conv_BoolToString` (`self.ReachedSplineEnd`)) " --- ") (`KismetStringLibrary.Concat_StrStr` "bullet distance: " (`KismetStringLibrary.Conv_DoubleToString` (`self.SplineDistance`)) " in front of arrow: " (`KismetStringLibrary.Conv_BoolToString` (> _dotproduct 0.0)))) true true (struct :`G` 0.66 :`B` 1.0 :`A` 1.0) 2.0 "bullet info")
  (if (`self.ReachedSplineEnd`)
    (if (< _dotproduct 0.0)
      (if (`KismetMathLibrary.InRange_FloatFloat` (`SplineComponent.GetDistanceAlongSplineAtSplineInputKey` _spline (`SplineComponent.FindInputKeyClosestToWorldLocation` _spline (`SceneComponent.K2_GetComponentLocation` (`self.BulletMesh`)))) 0.0 (`SplineComponent.GetSplineLength` _spline) false false) :!label _label
        (`self.SplineAlign`)
        (goto _label_2 :!via `Reset`)
        (else
          _)))
    (else
      (`self.TestIfAtFirstBox`)
      (goto _label)))
  (`self.TestIfReachedSplineEnd`)
  (`|ExecutionSequence`
    (:`then_0`
      (`/Engine/EditorBlueprintResources/StandardMacros.DoOnce` false :!label _label_2 ; Had issues where bullets would try aligning far past when it needed to, causing stops and other issues
        (:`Completed`
          (`MovementComponent.SetPlaneConstraintNormal` (`self.ProjectileMovement`) (`.JustRemove Z` (`/Game/Blueprints/Object_MacroLibrary.VectorRemoveZ` (`SceneComponent.GetRightVector` _returnvalue))))
          (`self.SetVelocityExitSpline`))))
    (:`then_1`
      (if (> (* (`KismetMathLibrary.Vector_Distance` (`.JustRemove Z` (`/Game/Blueprints/Object_MacroLibrary.VectorRemoveZ` (`SceneComponent.K2_GetComponentLocation` _returnvalue))) (`.JustRemove Z` (`/Game/Blueprints/Object_MacroLibrary.VectorRemoveZ` (`SceneComponent.K2_GetComponentLocation` (`self.BulletMesh`))))) _dotproduct) 300.0)
        (set `self.TurnSpline` null)
        (`KismetSystemLibrary.PrintString` "Bullet - Spline Reference Removed" true true (struct :`R` 1.0 :`G` 0.290672 :`B` 0.644788 :`A` 1.0))))))

(event `self.ReceiveTick`
  (params (DeltaSeconds :type "Float (single-precision)"))
  (`self.SetBulletZLocationTrace`)
  (`self.TurnSpline`
    (:`then`
      (`self.SetToSpline`))
    (:`else`)))

(event `TestIfReachedSplineEnd`
  (bind _atfirstbox (`self.AtFirstBox`))
  (bind _turnspline (`self.TurnSpline`))
  (bind _returnvalue (> (`self.GetDotProduct`) 0.0))
  (bind _returnvalue_2 (> (`KismetMathLibrary.Vector_Distance` (`.JustRemove Z` (`/Game/Blueprints/Object_MacroLibrary.VectorRemoveZ` (`SceneComponent.K2_GetComponentLocation` (select `bool` _atfirstbox :`false` (`/Game/Blueprints/SplineStuff/TurnSpline.ArrowB` _turnspline) :`true` (`/Game/Blueprints/SplineStuff/TurnSpline.ArrowA` _turnspline))))) (`.JustRemove Z` (`/Game/Blueprints/Object_MacroLibrary.VectorRemoveZ` (`SceneComponent.K2_GetComponentLocation` (`self.BulletMesh`))))) 50.0))
  (`self.TurnSpline`
    (:`then`
      (bind _output_get (set `self.ReachedSplineEnd` (or (and _atfirstbox _returnvalue_2 _returnvalue) (and (not _atfirstbox) _returnvalue_2 _returnvalue)))))
    (:`else`)))

(event `SetVelocityExitSpline`
  (bind _turnspline (`self.TurnSpline`))
  (set `MovementComponent.Velocity` (* (select `bool` (`self.AtFirstBox`) :`false` (`SceneComponent.GetForwardVector` (`/Game/Blueprints/SplineStuff/TurnSpline.ArrowB` _turnspline)) :`true` (`SceneComponent.GetForwardVector` (`/Game/Blueprints/SplineStuff/TurnSpline.ArrowA` _turnspline))) (`self.TargetSpeed`) (`/Game/Blueprints/Object_MacroLibrary.BoolFloatFlipper` 1.0 (`|EnumEquality` (`self.Direction`) "NewEnumerator1"))) (`self.ProjectileMovement`)))

(event `SetBulletRotationByVelocity`
  (`SceneComponent.K2_SetWorldRotation` (`self.BulletMesh`) (`KismetMathLibrary.FindLookAtRotation` (0.0 0.0 0.0) (`MovementComponent.Velocity` (`self.ProjectileMovement`))) false false))

(event `self.BulletMesh.OnComponentBeginOverlap`
  (params (OverlappedComponent :type "PrimitiveComponent Object Reference") (OtherActor :type "Actor Object Reference") (OtherComp :type "PrimitiveComponent Object Reference") (OtherBodyIndex :type Integer) (bFromSweep :type Boolean) (SweepResult :type "HitResult Structure (by ref)"))
  (bind _atfirstbox (`self.AtFirstBox`))
  (bind _returnvalue (not (`self.AtFirstBox`)))
  (bind _asturn_spline (cast `/Game/Blueprints/SplineStuff/TurnSpline` OtherActor))
  (if (== OtherComp (`/Game/Blueprints/SplineStuff/TurnSpline.BoxA` _asturn_spline))
    ;[1 1 1] overlapped with left Box for Spline
    (set `self.ReachedSplineEnd` false)
    (`MovementComponent.SetPlaneConstraintNormal` (`self.ProjectileMovement`) (`SceneComponent.GetRightVector` (`/Game/Blueprints/SplineStuff/TurnSpline.ArrowA` _asturn_spline)))
    (bind _turnspline (`self.TurnSpline`)
      (:`then`
        (if (or (!= _turnspline _asturn_spline) _returnvalue)
          (`KismetSystemLibrary.PrintString` (select `bool` _returnvalue :`true` "reseting, thinks still at 2nd box"))
          (set `self.SplineDistance` 0.0 :!label _label_3)
          (set `self.TurnSpline` _asturn_spline)))
      (:`else`
        (goto _label_3)))
    (elif (== OtherComp (`/Game/Blueprints/SplineStuff/TurnSpline.BoxB` _asturn_spline))
      ;[1 0.5487 0.6634] overlap with right spline box
      (set `self.ReachedSplineEnd` false)
      (`MovementComponent.SetPlaneConstraintNormal` (`self.ProjectileMovement`) (`SceneComponent.GetRightVector` (`/Game/Blueprints/SplineStuff/TurnSpline.ArrowB` _asturn_spline)))
      (bind _turnspline_2 (`self.TurnSpline`)
        (:`then`
          (if (or _atfirstbox (!= _turnspline_2 _asturn_spline))
            (`KismetSystemLibrary.PrintString` (select `bool` _atfirstbox :`true` "reseting, thinks still at first box"))
            (set `self.SplineDistance` (`SplineComponent.GetSplineLength` (`/Game/Blueprints/SplineStuff/TurnSpline.Spline` _asturn_spline)) :!label _label_4)
            (set `self.TurnSpline` _asturn_spline)))
        (:`else`
          (goto _label_4))))))

(event `BulletBounced`
  (`self.RemoveBulletFromGame`))

(event `self.ProjectileMovement.OnProjectileBounce`
  (params (ImpactResult :type "HitResult Structure (by ref)") (ImpactVelocity :type "Vector Structure (by ref)"))
  (`self.BulletBounced`))

(fn `UserConstructionScript`)