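; Player grenade, a child projectile of a bullet class, thrown in an arc and spawning a player explosion when it bounces or deals damage.
; Initial velocity follows the ground slope found by a downward trace, plus a lift along the surface normal, or forward and up without a hit.
; On turn splines it redirects horizontal velocity along the path and exit arrows, preserving vertical speed.
; Inherited height-trace and rotation-by-velocity events are emptied for optimization.
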(event `self.SetInitialVelocity`
  (bind _bulletmesh (`self.BulletMesh`))
  (bind _velocity (`MovementComponent.Velocity` (`self.ProjectileMovement`)))
  (bind (_returnvalue_roll _returnvalue_pitch _returnvalue_yaw) (`KismetMathLibrary.BreakRotator` (`KismetMathLibrary.FindLookAtRotation` (0.0 0.0 0.0) _velocity)))
  (bind _returnvalue (+ (* (`SceneComponent.GetForwardVector` _bulletmesh) 100.0) (`SceneComponent.K2_GetComponentLocation` _bulletmesh)))
  (bind (_outhit _returnvalue_2) (`KismetSystemLibrary.LineTraceSingleForObjects` :`Start` _returnvalue :`End` (- _returnvalue (* (`SceneComponent.GetUpVector` (`self.BulletMesh`)) 1200.0)) :`ObjectTypes` (`|MakeArray` "ObjectTypeQuery1" :!type "EObjectTypeQuery Enum") :`DrawTime` 1.0))
  (if _returnvalue_2
    (set `MovementComponent.Velocity` (+ (* (`KismetMathLibrary.Normal` (`KismetMathLibrary.GetForwardVector` (`KismetMathLibrary.MakeRotator` _returnvalue_roll (.pitch (`KismetMathLibrary.Conv_VectorToRotator` (+ (`KismetMathLibrary.RotateAngleAxis` (`.ImpactNormal` (`GameplayStatics.BreakHitResult` _outhit)) 90.0 (`KismetMathLibrary.GreaterGreater_VectorRotator` (`KismetMathLibrary.Normal` _velocity) (struct :`Yaw` 90.0))) (`KismetMathLibrary.Conv_RotatorToVector` (`SceneComponent.K2_GetComponentRotation` (`self.BulletMesh`)))))) _returnvalue_yaw))) (`self.TargetSpeed`)) (* (`.ImpactNormal` (`GameplayStatics.BreakHitResult` _outhit)) (`self.ThrowVerticlePower`))) (`self.ProjectileMovement`))
    (else
      (set `MovementComponent.Velocity` (+ (* (`KismetMathLibrary.Normal` (`KismetMathLibrary.GetForwardVector` (`SceneComponent.K2_GetComponentRotation` (`self.BulletMesh`)))) (`self.TargetSpeed`)) (`KismetMathLibrary.MakeVector` 0.0 0.0 (`self.ThrowVerticlePower`))) (`self.ProjectileMovement`))
      (`KismetSystemLibrary.DrawDebugArrow` (0.0 0.0 0.0)))))

(event `self.SetBulletZLocationTrace`
  ;[1 1 1] Overrides events by having them not do anything, since we do not their functionality for this child class. Optimization is 🔑
)

(event `self.SetBulletRotationByVelocity`
  ;[1 1 1] Overrides events by having them not do anything, since we do not their functionality for this child class. Optimization is 🔑
)

(event `self.ReceiveBeginPlay`
  (`parent.ReceiveBeginPlay`))

(event `self.ReceiveTick`
  (params (DeltaSeconds :type "Float (single-precision)"))
  (`parent.ReceiveTick` DeltaSeconds)
  (`KismetSystemLibrary.PrintString` (`KismetStringLibrary.Concat_StrStr` "bullet grende: " (`KismetStringLibrary.Conv_RotatorToString` (`SceneComponent.K2_GetComponentRotation` (`self.BulletMesh`))))))

(event `self.SetVelocityOnSpline`
  (params (Velocity :type "Vector Structure"))
  (bind _returnvalue (`SplineComponent.GetSplineLength` (`/Game/Blueprints/SplineStuff/TurnSpline.Spline` (`self.TurnSpline`))))
  (set `MovementComponent.Velocity` (+ (* (`KismetMathLibrary.Normal` (`KismetMathLibrary.GetForwardVector` (`KismetMathLibrary.FindLookAtRotation` (`.JustRemove Z` (`/Game/Blueprints/Object_MacroLibrary.VectorRemoveZ` (`SplineComponent.GetLocationAtDistanceAlongSpline` (`/Game/Blueprints/SplineStuff/TurnSpline.Spline` (`self.TurnSpline`)) (`self.SplineDistance`) "World"))) (`.JustRemove Z` (`/Game/Blueprints/Object_MacroLibrary.VectorRemoveZ` (`SplineComponent.GetLocationAtDistanceAlongSpline` (`/Game/Blueprints/SplineStuff/TurnSpline.Spline` (`self.TurnSpline`)) (`KismetMathLibrary.FClamp` (+ (`KismetMathLibrary.FClamp` (`self.SplineDistance`) 3.0 (- _returnvalue 4.0)) (`/Game/Blueprints/Object_MacroLibrary.BoolFloatFlipper` 55.0 (`|EnumEquality` (`self.Direction`) "NewEnumerator1"))) 0.0 _returnvalue) "World")))))) (`KismetMathLibrary.VSize` (`KismetMathLibrary.MakeVector` (.x (`MovementComponent.Velocity` (`self.ProjectileMovement`))) (.y (`MovementComponent.Velocity` (`self.ProjectileMovement`)))))) (`KismetMathLibrary.MakeVector` 0.0 0.0 (.z (`MovementComponent.Velocity` (`self.ProjectileMovement`))))) (`self.ProjectileMovement`)))

(event `self.ProjectileMovement.OnProjectileBounce`
  (params (ImpactResult :type "HitResult Structure (by ref)") (ImpactVelocity :type "Vector Structure (by ref)"))
  ;[1 1 1] Hit wall/ground
  (`self.RemoveBulletFromGame`))

(event `self.SetVelocityExitSpline`
  (bind _turnspline (`self.TurnSpline`))
  (set `MovementComponent.Velocity` (+ (* (`KismetMathLibrary.Normal` (select `bool` (`self.AtFirstBox`) :`false` (`SceneComponent.GetForwardVector` (`/Game/Blueprints/SplineStuff/TurnSpline.ArrowB` _turnspline)) :`true` (`SceneComponent.GetForwardVector` (`/Game/Blueprints/SplineStuff/TurnSpline.ArrowA` _turnspline)))) (`KismetMathLibrary.VSize` (`KismetMathLibrary.MakeVector` (.x (`MovementComponent.Velocity` (`self.ProjectileMovement`))) (.y (`MovementComponent.Velocity` (`self.ProjectileMovement`))))) (`/Game/Blueprints/Object_MacroLibrary.BoolFloatFlipper` 1.0 (`|EnumEquality` (`self.Direction`) "NewEnumerator1"))) (`KismetMathLibrary.MakeVector` 0.0 0.0 (.z (`MovementComponent.Velocity` (`self.ProjectileMovement`))))) (`self.ProjectileMovement`)))

(event `/Game/Blueprints/Mechanics/HealthAndDamageInterface.DamageSuccessful`
  ;[1 0.2522 0.4851] Hit enemy
  (`self.RemoveBulletFromGame`))

(event `self.RemoveBulletFromGame`
  (`|SpawnActorFromClass` "/Game/Blueprints/Attacks/Explosion_Player.Explosion_Player_C" (`KismetMathLibrary.MakeTransform` (`self.K2_GetActorLocation`)) "Undefined" "MultiplyWithRoot" null self 150 null)
  (`self.K2_DestroyActor`))

(fn `UserConstructionScript`
  (`parent.UserConstructionScript`))