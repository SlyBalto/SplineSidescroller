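; Trigger actor that automatically moves the third-person character onto another spline, AutoSwitchTo, when it overlaps the box.
; If that differs from the current spline, it updates the character's spline and, when valid, calls SwitchToNewSpline at zero distance.
; It then sets forward rotation from a flattened spline tangent, looked up using a local spline direction as the world location.
; The construction script shows a billboard while no valid target is assigned.
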(event `self.Box.OnComponentBeginOverlap`
  (params (OverlappedComponent :type "PrimitiveComponent Object Reference") (OtherActor :type "Actor Object Reference") (OtherComp :type "PrimitiveComponent Object Reference") (OtherBodyIndex :type Integer) (bFromSweep :type Boolean) (SweepResult :type "HitResult Structure (by ref)"))
  (bind _autoswitchto (`self.AutoSwitchTo`))
  (bind _spline (`/Game/Blueprints/SplineStuff/TurnSpline.Spline` _autoswitchto))
  (bind _asbp_third_person_character (cast `/Game/Blueprints/Player/BP_ThirdPersonCharacter` OtherActor))
  (if (!= (`.CurrentSpline_9_ADBB94374E7CEDCE5F0EFBBE750C5B05` (break `/Game/Blueprints/Mechanics/SplineInfo` (`/Game/Blueprints/Player/BP_ThirdPersonCharacter.SplineInfo` _asbp_third_person_character))) _autoswitchto)
    (`/Game/Blueprints/Player/BP_ThirdPersonCharacter.UpdateCurrentSpline` _asbp_third_person_character (`self.AutoSwitchTo`))
    (`self.AutoSwitchTo`
      (:`then`
        ;[1 1 1] may need to set the New Distance
        (`/Game/Blueprints/Player/BP_ThirdPersonCharacter.SwitchToNewSpline` _asbp_third_person_character 0.0 false 0.0)
        (bind _normalized (`/Game/Blueprints/Object_MacroLibrary.VectorRemoveZ` (`SplineComponent.FindTangentClosestToWorldLocation` _spline (`SplineComponent.GetDirectionAtDistanceAlongSpline` _spline (`SplineComponent.GetDistanceAlongSplineAtSplineInputKey` _spline (`SplineComponent.FindInputKeyClosestToWorldLocation` _spline (`self.K2_GetActorLocation` _asbp_third_person_character))) "Local") "World")))
        (`/Game/Blueprints/Player/BP_ThirdPersonCharacter.UpdateForwardRot` _asbp_third_person_character (`KismetMathLibrary.MakeRotationFromAxes` _normalized (`KismetMathLibrary.GreaterGreater_VectorRotator` _normalized (struct :`Yaw` 90.0)) (0.0 0.0 1.0))))
      (:`else`))))

(fn `UserConstructionScript`
  (`SceneComponent.SetVisibility` (`self.Billboard`) (not (`KismetSystemLibrary.IsValid` (`self.AutoSwitchTo`))) false))