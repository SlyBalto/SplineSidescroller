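; CameraRotateToggle is a trigger volume that changes how the third-person character's follow camera behaves on entry.
; Overlap toggles yaw inheritance, using the Arrow's direction as the fixed yaw, then enables spline lock or releases it on all toggles if no spline is assigned.
; While locked, Tick snaps the camera to the spline point nearest the player and takes yaw from its tangent.
; The construction script updates icons and arrow to preview the settings.
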(event `self.ReceiveTick`
  (params (DeltaSeconds :type "Float (single-precision)"))
  (bind _spline (`/Game/Blueprints/SplineStuff/CameraSpline.Spline` (`self.SplineCamUse`)))
  (`self.SplineCamUse`
    (:`then`
      (bind _player (`self.Player`)
        (:`then`
          (if (`self.PlayerCamFollowsSpline`)
            (bind _followcam (`/Game/Blueprints/Player/BP_ThirdPersonCharacter.FollowCam` _player))
            (bind _returnvalue (`SplineComponent.FindInputKeyClosestToWorldLocation` _spline (`self.K2_GetActorLocation` _player)))
            (`self.K2_SetActorLocation` _followcam (`SplineComponent.GetLocationAtDistanceAlongSpline` _spline (`SplineComponent.GetDistanceAlongSplineAtSplineInputKey` _spline _returnvalue) "World") false false)
            (bind (_returnvalue_roll _returnvalue_pitch _returnvalue_yaw) (`KismetMathLibrary.BreakRotator` (`KismetMathLibrary.FindLookAtRotation` (0.0 0.0 0.0) (`KismetMathLibrary.GreaterGreater_VectorRotator` (`SplineComponent.GetTangentAtSplineInputKey` _spline _returnvalue "World") (struct)))))
            (bind _output_get (set `/Game/Blueprints/FollowCam.TargetCameraZRotation` _returnvalue_yaw _followcam))
            (`KismetSystemLibrary.PrintString` (`KismetStringLibrary.Conv_DoubleToString` _output_get))
            (else
              (`self.K2_SetActorRelativeLocation` _followcam (0.0 0.0 0.0) false false))))
        (:`else`)))
    (:`else`)))

(event `self.Box.OnComponentBeginOverlap`
  (params (OverlappedComponent :type "PrimitiveComponent Object Reference") (OtherActor :type "Actor Object Reference") (OtherComp :type "PrimitiveComponent Object Reference") (OtherBodyIndex :type Integer) (bFromSweep :type Boolean) (SweepResult :type "HitResult Structure (by ref)"))
  (bind (_returnvalue_roll _returnvalue_pitch _returnvalue_yaw) (`KismetMathLibrary.BreakRotator` (`KismetMathLibrary.FindLookAtRotation` (0.0 0.0 0.0) (`SceneComponent.GetForwardVector` (`self.Arrow`)))))
  (bind _asbp_third_person_character (cast `/Game/Blueprints/Player/BP_ThirdPersonCharacter` OtherActor))
  (set `self.Player` _asbp_third_person_character)
  (`/Game/Blueprints/FollowCam.ToggleInheritYaw` (`/Game/Blueprints/Player/BP_ThirdPersonCharacter.FollowCam` _asbp_third_person_character) (`self.EnablesFollowCameraRotation`) _returnvalue_yaw)
  (`self.SplineCamUse`
    (:`then`
      (`self.ToggleLockCam` true))
    (:`else`
      (bind _outactors (`GameplayStatics.GetAllActorsOfClass` "CameraRotateToggle_C"))
      (`self.ToggleLockCam` _outactors false))))

(event `ToggleLockCam`
  (params (`Camera Follows Spline` :type Boolean))
  (set `self.PlayerCamFollowsSpline` `Camera Follows Spline`)
  (`self.Player`
    (:`then`)
    (:`else`)))

(fn `UserConstructionScript`
  (bind (_returnvalue_x _returnvalue_y) (`KismetMathLibrary.BreakVector` (`SceneComponent.K2_GetComponentLocation` (`self.Arrow`))))
  (`BillboardComponent.SetSprite` (`self.InfoIcon`) (select `bool` (`self.EnablesFollowCameraRotation`) :`false` "/Engine/EditorMaterials/Cascade/CASC_ModuleDisable.CASC_ModuleDisable" :`true` "/Engine/EditorMaterials/GreyCheck.GreyCheck" :!type "Texture2D Object Reference"))
  (`SceneComponent.K2_SetWorldLocation` (`self.InfoIcon`) (+ (`SceneComponent.K2_GetComponentLocation` (`self.cam icon`)) (0.0 0.0 37.0)) false false)
  (`SceneComponent.K2_SetWorldLocation` (`self.Arrow`) (`KismetMathLibrary.MakeVector` _returnvalue_x _returnvalue_y (.z (+ (`self.K2_GetActorLocation`) (0.0 0.0 100.0)))) false false)
  (`SceneComponent.SetVisibility` (`self.Arrow`) (not (`self.EnablesFollowCameraRotation`)) false)
  (`SceneComponent.SetVisibility` (`self.CameraLockIgnoreAxis`) (`KismetSystemLibrary.IsValid` (`self.SplineCamUse`)) false))