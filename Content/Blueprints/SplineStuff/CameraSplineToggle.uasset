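; Camera trigger for a spline-scroller that switches the view when the player character enters its box.
; On overlap it stores the player and blends to SplineCamera, or to the player's FollowCam if none is set.
; While ToggleLockCam's flag is on, Tick snaps FollowCam to the nearest SplineForCam point, derives target yaw from the tangent and prints it; otherwise it resets the relative location.
; The construction script updates editor icons and arrow.
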(event `self.ReceiveTick`
  (params (DeltaSeconds :type "Float (single-precision)"))
  (bind _spline (`/Game/Blueprints/SplineStuff/CameraSpline.Spline` (`self.SplineForCam`)))
  (`self.SplineForCam`
    (:`then`
      (bind _player (`self.Player`)
        (:`then`
          (if (`self.PlayerCamFollowsSpline`)
            (bind _followcam (`/Game/Blueprints/Player/SplinescrollerCharacter.FollowCam` _player))
            (bind _returnvalue (`SplineComponent.FindInputKeyClosestToWorldLocation` _spline (`self.K2_GetActorLocation` _player)))
            (`self.K2_SetActorLocation` _followcam (`SplineComponent.GetLocationAtDistanceAlongSpline` _spline (`SplineComponent.GetDistanceAlongSplineAtSplineInputKey` _spline _returnvalue) "World") false false)
            (bind (_returnvalue_roll _returnvalue_pitch _returnvalue_yaw) (`KismetMathLibrary.BreakRotator` (`KismetMathLibrary.FindLookAtRotation` (0.0 0.0 0.0) (`KismetMathLibrary.GreaterGreater_VectorRotator` (`SplineComponent.GetTangentAtSplineInputKey` _spline _returnvalue "World")))))
            (bind _output_get (set `/Game/Blueprints/Player/Camera/FollowCam.TargetCameraZRotation` _returnvalue_yaw _followcam))
            (`KismetSystemLibrary.PrintString` (`KismetStringLibrary.Conv_DoubleToString` _output_get))
            (else
              (`self.K2_SetActorRelativeLocation` _followcam (0.0 0.0 0.0) false false))))
        (:`else`)))
    (:`else`)))

(event `self.Box.OnComponentBeginOverlap`
  (params (OverlappedComponent :type "PrimitiveComponent Object Reference") (OtherActor :type "Actor Object Reference") (OtherComp :type "PrimitiveComponent Object Reference") (OtherBodyIndex :type Integer) (bFromSweep :type Boolean) (SweepResult :type "HitResult Structure (by ref)"))
  (bind _assplinescroller_character (cast `/Game/Blueprints/Player/SplinescrollerCharacter` OtherActor))
  (bind _output_get (set `self.Player` _assplinescroller_character))
  (bind _splinecamera (`self.SplineCamera`)
    (:`then`
      (`PlayerController.SetViewTargetWithBlend` (`GameplayStatics.GetPlayerController` 0) _splinecamera 0.0 "VTBlend_Linear" 0.0 false))
    (:`else`
      (`PlayerController.SetViewTargetWithBlend` (`GameplayStatics.GetPlayerController` 0) (`/Game/Blueprints/Player/SplinescrollerCharacter.FollowCam` _output_get) 0.0 "VTBlend_Linear" 0.0 false))))

(event `ToggleLockCam`
  (params (`Camera Follows Spline` :type Boolean))
  (set `self.PlayerCamFollowsSpline` `Camera Follows Spline`)
  (`self.Player`
    (:`then`)
    (:`else`)))

(fn `UserConstructionScript`
  (bind (_returnvalue_x _returnvalue_y) (`KismetMathLibrary.BreakVector` (`SceneComponent.K2_GetComponentLocation` (`self.Arrow`))))
  (`BillboardComponent.SetSprite` (`self.InfoIcon`) (select `bool` (`self.UseAltCam`) :`false` "/Engine/EditorMaterials/Cascade/CASC_ModuleDisable.CASC_ModuleDisable" :`true` "/Engine/EditorMaterials/GreyCheck.GreyCheck" :!type "Texture2D Object Reference"))
  (`SceneComponent.K2_SetWorldLocation` (`self.InfoIcon`) (+ (`SceneComponent.K2_GetComponentLocation` (`self.cam icon`)) (0.0 0.0 37.0)) false false)
  (`SceneComponent.K2_SetWorldLocation` (`self.Arrow`) (`KismetMathLibrary.MakeVector` _returnvalue_x _returnvalue_y (.z (+ (`self.K2_GetActorLocation`) (0.0 0.0 100.0)))) false false)
  (`SceneComponent.SetVisibility` (`self.Arrow`) (not (`self.UseAltCam`)) false)
  (`SceneComponent.SetVisibility` (`self.CameraLockIgnoreAxis`) (`KismetSystemLibrary.IsValid` (`self.SplineForCam`)) false))