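; AltCamSpline is an actor tied to a camera spline that keeps turning to face the player, apparently as an alternate spline camera.
; The construction script snaps it to the midpoint of the referenced CamSpline's spline, measured by distance in world space.
; On Tick it sets its rotation directly to look at the Player's location, with no smoothing, while its position stays where construction placed it.
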(event `self.ReceiveTick`
  (params (DeltaSeconds :type "Float (single-precision)"))
  (bind _player (`self.Player`)
    (:`then`
      (`self.K2_SetActorRotation` (`KismetMathLibrary.FindLookAtRotation` (`self.K2_GetActorLocation`) (`self.K2_GetActorLocation` _player))))
    (:`else`)))

(fn `UserConstructionScript`
  (bind _spline (`/Game/Blueprints/SplineStuff/CameraSpline.Spline` (`self.CamSpline`)))
  (`self.CamSpline`
    (:`then`
      (`self.K2_SetActorLocation` (`SplineComponent.GetLocationAtDistanceAlongSpline` _spline (/ (`SplineComponent.GetSplineLength` _spline) 2.0) "World")))
    (:`else`)))