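; TurnSpline is a spline path actor with a query-only box at each end, presumably for turns; no overlap logic lives here.
; The construction script fits both boxes and arrows to the spline ends, shows X markers for disabled states, and optionally adds distance markers or test spline meshes.
; Box collision requires both the spline and that box to be enabled, switchable at runtime through events including SetActiveGeneral.
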(event `UpdateBoxesEnabled`
  (params (`Enable Box A` :type Boolean) (`Enable Box B` :type Boolean))
  (bind _output_get (set `self.Enable Box A` `Enable Box A`))
  (`PrimitiveComponent.SetCollisionEnabled` (`self.BoxA`) (select `bool` (and _output_get (`self.SplineEnabled`)) :`false` "NoCollision" :`true` "QueryOnly" :!type "ECollisionEnabled Enum"))
  (bind _output_get_2 (set `self.Enable Box B` `Enable Box B`))
  (`PrimitiveComponent.SetCollisionEnabled` (`self.BoxB`) (select `bool` (and _output_get_2 (`self.SplineEnabled`)) :`false` "NoCollision" :`true` "QueryOnly" :!type "ECollisionEnabled Enum")))

(event `self.ReceiveBeginPlay`
  (`self.ToggleSplineEnabled` (`self.SplineEnabled`))
  (`self.UpdateBoxesEnabled` (`self.Enable Box A`) (`self.Enable Box B`)))

(event `ToggleSplineEnabled`
  (params (Enabled :type Boolean))
  (bind _output_get (set `self.SplineEnabled` Enabled))
  (if _output_get
    (`self.UpdateBoxesEnabled` (`self.Enable Box A`) (`self.Enable Box B`))
    (else
      (`PrimitiveComponent.SetCollisionEnabled` (`self.BoxB`) "NoCollision")
      (`PrimitiveComponent.SetCollisionEnabled` (`self.BoxA`) "NoCollision"))))

(event `/Game/Blueprints/Mechanics/GeneralActivateInterface.SetActiveGeneral`
  (params (Active :type Boolean))
  (`self.ToggleSplineEnabled` Active))

(event `MakeTestSplineMesh`
  (bind _spline (`self.Spline`))
  (`KismetArrayLibrary.Array_Clear` (`self.SplineMeshes`))
  (for _index (range (+ (- (`SplineComponent.GetNumberOfSplinePoints` (`self.Spline`)) 2) 1))
    (bind _returnvalue (`AddComponent|NODE_AddSplineMeshComponent-1` :`bManualAttachment` true))
    (`KismetArrayLibrary.Array_Add` (`self.SplineMeshes`) _returnvalue)
    (bind (_location _tangent) (`SplineComponent.GetLocationAndTangentAtSplinePoint` _spline _index "Local"))
    (bind (_location_2 _tangent_2) (`SplineComponent.GetLocationAndTangentAtSplinePoint` _spline (+ _index 1) "Local"))
    (`SplineMeshComponent.SetStartAndEnd` _returnvalue _location _tangent _location_2 _tangent_2 true)
    (`PrimitiveComponent.SetCollisionEnabled` _returnvalue "QueryAndPhysics")
    (`SceneComponent.K2_AttachToComponent` _returnvalue (`self.DefaultSceneRoot`) "None" "KeepRelative" "KeepRelative" "KeepRelative" true)))

(event `/Game/Blueprints/Editor/EditorDebugInterface.ToggleSetDebugAsHidden`
  (params (HideDebug :type Boolean))
  (`SceneComponent.SetHiddenInGame` (`self.BoxB`) HideDebug false)
  (`SceneComponent.SetHiddenInGame` (`self.BoxA`) HideDebug false))

(fn `UserConstructionScript`
  (bind _boxa (`self.BoxA`))
  (bind _spline (`self.Spline`))
  (bind _spline_2 (`self.Spline`))
  (bind _spline_3 (`self.Spline`))
  (bind _boxb (`self.BoxB`))
  (bind _boxa_2 (`self.BoxA`))
  (bind (_returnvalue_x _returnvalue_y _returnvalue_z) (`KismetMathLibrary.BreakVector` (`BoxComponent.GetScaledBoxExtent` _boxa_2)))
  (bind _returnvalue_x_2 (`KismetMathLibrary.BreakVector` (`BoxComponent.GetScaledBoxExtent` (`self.BoxB`))))
  (bind (_returnvalue_x_3 _returnvalue_y_2 _returnvalue_z_2) (`KismetMathLibrary.BreakVector` (`BoxComponent.GetScaledBoxExtent` (`self.BoxB`))))
  (bind _returnvalue (`SplineComponent.GetRotationAtTime` _spline 0.0 "World" false))
  (bind _returnvalue_2 (`SplineComponent.GetRotationAtTime` _spline_2 1.0 "World" false))
  (bind _returnvalue_3 (+ (- 0.0 (`self.Height A`)) 50.0))
  (`SceneComponent.SetVisibility` (`self.Spline Enabled X A`) (not (`self.SplineEnabled`)) false)
  (`SceneComponent.SetVisibility` (`self.Spline Enabled X B`) (not (`self.SplineEnabled`)) false)
  (`SceneComponent.SetVisibility` (`self.X Overlap A`) (not (`self.Enable Box A`)) false)
  (`SceneComponent.SetVisibility` (`self.X Overlap B`) (not (`self.Enable Box B`)) false)
  (`|ExecutionSequence`
    (:`then_0`
      (`SceneComponent.K2_SetRelativeLocation` (`self.Spline`) (`KismetMathLibrary.MakeVector` 0.0 0.0 (select `bool` (`self.DisableSplineOffset`) :`false` 100.0)) false false)
      (`BoxComponent.SetBoxExtent` _boxa (`KismetMathLibrary.MakeVector` 75.0 25.0 (`self.Height A`)) true)
      (`BoxComponent.SetBoxExtent` (`self.BoxB`) (`KismetMathLibrary.MakeVector` 75.0 25.0 (`self.Height B`)) true)
      (`SceneComponent.SetWorldScale3D` _boxa (1.0 1.0 1.0))
      (`SceneComponent.SetWorldScale3D` (`self.BoxB`) (1.0 1.0 1.0))
      (`SceneComponent.K2_SetWorldLocation` _boxb (+ (`SplineComponent.GetLocationAtDistanceAlongSpline` _spline_2 (`SplineComponent.GetSplineLength` _spline_2) "World") (* (`KismetMathLibrary.GetForwardVector` _returnvalue_2) _returnvalue_x_3) (`KismetMathLibrary.MakeVector` 0.0 0.0 _returnvalue_z_2) (`KismetMathLibrary.MakeVector` 0.0 0.0 (select `bool` (`self.DisableSplineOffset`) :`false` -100.0))) false false)
      (`SceneComponent.K2_SetWorldRotation` _boxb _returnvalue_2 false false)
      (`SceneComponent.K2_SetWorldLocation` _boxa_2 (+ (`SplineComponent.GetLocationAtDistanceAlongSpline` _spline 0.0 "World") (* (`KismetMathLibrary.GetForwardVector` _returnvalue) (* _returnvalue_x_2 -1.0)) (`KismetMathLibrary.MakeVector` 0.0 0.0 _returnvalue_z) (`KismetMathLibrary.MakeVector` 0.0 0.0 (select `bool` (`self.DisableSplineOffset`) :`false` -100.0))) false false)
      (`SceneComponent.K2_SetWorldRotation` _boxa_2 _returnvalue false false)
      (`SceneComponent.K2_SetRelativeLocation` (`self.ArrowA`) (`KismetMathLibrary.MakeVector` 100.0 0.0 _returnvalue_3) false false)
      (`SceneComponent.K2_SetRelativeLocation` (`self.ArrowB`) (`KismetMathLibrary.MakeVector` -100.0 0.0 _returnvalue_3) false false)
      (if (`self.DistanceDebug`)
        (`|ExecutionSequence`
          (:`then_0`
            (goto _label :!via `Reset`))
          (:`then_1`
            (bind _counter (`/Engine/EditorBlueprintResources/StandardMacros.Do N` 99 :!label _label)
              (:`Exit`
                (bind _returnvalue_4 (`KismetMathLibrary.Conv_IntToDouble` (* (- _counter 1) 100)))
                (if (< _returnvalue_4 (`SplineComponent.GetSplineLength` _spline_3))
                  (bind _returnvalue_5 (`AddComponent|NODE_AddStaticMeshComponent-0` :`bManualAttachment` true :`RelativeTransform` (`KismetMathLibrary.MakeTransform` (0.0 0.0 0.0) (struct) (`KismetMathLibrary.Conv_DoubleToVector` 0.2))))
                  (`SceneComponent.K2_SetWorldLocation` _returnvalue_5 (+ (`SplineComponent.GetLocationAtDistanceAlongSpline` _spline_3 _returnvalue_4 "World") (0.0 0.0 100.0)) false false)
                  (goto _label))))))))
    (:`then_2`
      (if (`self.MakeTestMesh`)
        (`self.MakeTestSplineMesh`)))))