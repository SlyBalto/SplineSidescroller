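; Spline turn piece that shapes itself in the editor into a 90 or 180 degree turn, left or right.
; The construction script grid-snaps the radius, then places points and tangents scaled by a multiplier to form the arc, flipping Y for direction.
; A DoOnce guards adding the third point for 180 degree turns, which is removed otherwise.
; The parent construction script runs after the spline is shaped.
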(fn `UserConstructionScript`
  (bind _radiususe (`self.GetTurnRadius`))
  (bind _spline (`self.Spline`))
  (bind _spline_2 (`self.Spline`))
  (bind _returnvalue (`KismetMathLibrary.MakeVector` (* (`self.GetTurnRadius`) (`self.Multi`) -1.0)))
  (bind _returnvalue_2 (* (`/Game/Blueprints/GameManagement/Object_MacroLibrary.BoolFloatFlipper` _radiususe (`self.TurnRight`)) (`self.Multi`)))
  (set `self.TurnRadius` (`KismetMathLibrary.GridSnap_Float` (`self.TurnRadius`) 50.0))
  (`SplineComponent.SetTangentsAtSplinePoint` (`self.Spline`) 0 (`KismetMathLibrary.MakeVector` 0.0) (`KismetMathLibrary.MakeVector` (* (`self.GetTurnRadius`) (`self.Multi`))) "Local" false)
  (`SplineComponent.SetTangentsAtSplinePoint` _spline 1 (`KismetMathLibrary.MakeVector` 0.0 _returnvalue_2) (`KismetMathLibrary.MakeVector` 0.0 (select `bool` (`self.180DegreesTurn`) :`true` _returnvalue_2)) "Local" false)
  (`SplineComponent.SetLocationAtSplinePoint` _spline 1 (`KismetMathLibrary.MakeVector` _radiususe (`/Game/Blueprints/GameManagement/Object_MacroLibrary.BoolFloatFlipper` _radiususe (`self.TurnRight`))) "Local" true)
  (if (`self.180DegreesTurn`)
    (`/Engine/EditorBlueprintResources/StandardMacros.DoOnce` false :!label _label
      (:`Completed`
        (`SplineComponent.AddPoint` _spline_2 (make `SplinePoint` 2.0 (`KismetMathLibrary.MakeVector` 0.0 (`/Game/Blueprints/GameManagement/Object_MacroLibrary.BoolFloatFlipper` (* (`self.GetTurnRadius`) 2.0) (`self.TurnRight`))) _returnvalue _returnvalue (struct) (1.0 1.0 1.0) "CurveCustomTangent") true)))
    (else
      (`|ExecutionSequence`
        (:`then_0`
          (goto _label :!via `Reset`))
        (:`then_1`
          (`SplineComponent.RemoveSplinePoint` _spline_2 2 true)))))
  (`parent.UserConstructionScript`))