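; Health component that manages an actor's health, death, revival, team-based overlap damage and post-hit invincibility.
; HealthOverlapTest reads opposing DamageComponents and calls TakeDamage, which clamps health and messages owner and attacker.
; Optional invincibility blinks a component on Tick and lasts while enemy damage actors overlap a check component, repolled through a recursive delay.
; DamageFlash creates dynamic materials once, then briefly pulses their Damaged parameter.
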(event `self.ReceiveTick`
  (params (DeltaSeconds :type "Float (single-precision)"))
  (bind _compforinvicibility (`self.CompForInvicibility`)
    (:`then`
      (if (`self.Invincible`)
        (bind _isa (`/Engine/EditorBlueprintResources/StandardMacros.FlipFlop`)
          (:`A`
            _)
          (:`B`
            _))
        (`SceneComponent.SetVisibility` _compforinvicibility _isa false)))
    (:`else`)))

(event `TryInvicibleStop`
  (`KismetSystemLibrary.Delay` 0.2)
  (bind _outactors (`KismetSystemLibrary.ComponentOverlapActors` (`self.CompCheckOverlapInvicible`) (`KismetMathLibrary.MakeTransform` (0.0 0.0 0.0)) (`|MakeArray` "ObjectTypeQuery2" :!type "EObjectTypeQuery Enum") :!label _label))
  (for _array_element _outactors
    (bind _returnvalue (`Actor.GetComponentByClass` _array_element "/Game/Blueprints/Mechanics/DamageComponent.DamageComponent_C"))
    (`/Engine/EditorBlueprintResources/StandardMacros.IsValid` _returnvalue
      (:`Is Valid`
        (if (!= (`/Game/Blueprints/Mechanics/DamageComponent.Team` _returnvalue) (`self.Team`))
          (`|ExecutionSequence`
            (:`then_0`
              (break))
            (:`then_1`
              (`self.TryInvicibleStop`)))))))
  (set `self.Invincible` false)
  (bind _compforinvicibility (`self.CompForInvicibility`)
    (:`then`
      (`SceneComponent.SetVisibility` _compforinvicibility true false))
    (:`else`)))

(event `StartTempInvincibility`
  (set `self.Invincible` true)
  (goto _label))

(event `UpdateMaxHealth`
  (params (NewMaxHealth :type Integer) (`Also Fully Heal` :type Boolean :default true))
  (bind _output_get (set `self.MaxHealth` NewMaxHealth))
  (if `Also Fully Heal`
    (`self.Heal` _output_get)))

(event `Revive`
  (`self.Heal` (`self.MaxHealth`))
  (set `self.Dead` false))

(event `TakeDamage`
  (params (Damage :type Integer) (AttackingActor :type "Actor Object Reference"))
  (if (and (not (`self.Dead`)) (not (`self.Invincible`)))
    (bind _output_get (set `self.CurrentHealth` (`KismetMathLibrary.Clamp` (- (`self.CurrentHealth`) Damage) 0 (`self.MaxHealth`))))
    (bind _output_get_2 (set `self.Dead` (<= _output_get 0)))
    (message `/Game/Blueprints/Mechanics/HealthAndDamageInterface.TookDamage` (`self.GetOwner`) _output_get_2 AttackingActor (`self.CurrentHealth`) (/ (`KismetMathLibrary.Conv_IntToDouble` (`self.CurrentHealth`)) (`KismetMathLibrary.Conv_IntToDouble` (`self.MaxHealth`)))) ; Actors with a Damage Interface can implement this event\nfor custom functionality after taking damage. This also gives\nthe actor helpful information.
    (`|ExecutionSequence`
      (:`then_0`
        (`/Engine/EditorBlueprintResources/StandardMacros.IsValid` AttackingActor
          (:`Is Valid`
            (message `/Game/Blueprints/Mechanics/HealthAndDamageInterface.DamageSuccessful` AttackingActor)
            (`KismetSystemLibrary.PrintString` "SENDIN OUT SUCC" true true (struct :`G` 1.0 :`B` 0.698992 :`A` 1.0)))))
      (:`then_1`
        (if (and (not _output_get_2) (`self.InvicibleAfterDamage`))
          (`self.StartTempInvincibility`))))))

(event `Heal`
  (params (`Heal Amount` :type Integer))
  (set `self.CurrentHealth` (`KismetMathLibrary.Clamp` (+ (`self.CurrentHealth`) `Heal Amount`) 0 (`self.MaxHealth`))))

(event `self.ReceiveBeginPlay`
  (set `self.MaxHealth` (`self.CurrentHealth`)))

(event `HealthOverlapTest`
  (params (CompOverlappedWith :type "ActorComponent Object Reference"))
  (bind _returnvalue (`self.GetOwner` CompOverlappedWith))
  (bind _returnvalue_2 (`Actor.GetComponentByClass` _returnvalue "/Game/Blueprints/Mechanics/DamageComponent.DamageComponent_C"))
  (`/Engine/EditorBlueprintResources/StandardMacros.IsValid` _returnvalue_2
    (:`Is Valid`
      (if (!= (`self.Team`) (`/Game/Blueprints/Mechanics/DamageComponent.Team` _returnvalue_2))
        (`self.TakeDamage` (`/Game/Blueprints/Mechanics/DamageComponent.DamageStrength` _returnvalue_2) _returnvalue)))))

(event `DamageFlash`
  (params (CompToFlash :type "PrimitiveComponent Object Reference"))
  (`|ExecutionSequence`
    (:`then_0`
      (`/Engine/EditorBlueprintResources/StandardMacros.DoOnce` false
        (:`Completed`
          (for _index (range (`PrimitiveComponent.GetNumMaterials` CompToFlash))
            (bind _returnvalue (`PrimitiveComponent.CreateDynamicMaterialInstance` CompToFlash _index (`PrimitiveComponent.GetMaterial` CompToFlash _index) "None"))
            (`KismetArrayLibrary.Array_Add` (`self.MaterialList`) _returnvalue)))))
    (:`then_1`
      (for _array_element (`self.MaterialList`)
        (`MaterialInstanceDynamic.SetScalarParameterValue` _array_element "Damaged" 1.0))
      (`KismetSystemLibrary.RetriggerableDelay` 0.2)
      (for _array_element_2 (`self.MaterialList`)
        (`MaterialInstanceDynamic.SetScalarParameterValue` _array_element_2 "Damaged" 0.0))
      (`KismetSystemLibrary.Delay` 0.2))))