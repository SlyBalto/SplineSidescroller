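; A box trigger volume that enables or disables a list of actors when the player's third-person character enters it.
; On overlap, it sends SetActiveGeneralMessage with its Enabling flag to every entry in ActorsToEnable.
; The construction script uses SwapEnabled as a self-resetting editor switch to flip Enabling, and sets the icon sprite to show the current mode.
; A debug event toggles the box's in-game visibility, including its child components.
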(event `self.Box.OnComponentBeginOverlap`
  (params (OverlappedComponent :type "PrimitiveComponent Object Reference") (OtherActor :type "Actor Object Reference") (OtherComp :type "PrimitiveComponent Object Reference") (OtherBodyIndex :type Integer) (bFromSweep :type Boolean) (SweepResult :type "HitResult Structure (by ref)"))
  (cast `/Game/Blueprints/Player/BP_ThirdPersonCharacter` OtherActor)
  (for _array_element (`self.ActorsToEnable`)
    (message `/Game/Blueprints/Mechanics/GeneralActivateInterface.SetActiveGeneral` _array_element (`self.Enabling?`))))

(event `/Game/Blueprints/Editor/EditorDebugInterface.ToggleSetDebugAsHidden`
  (params (HideDebug :type Boolean))
  (`SceneComponent.SetHiddenInGame` (`self.Box`) HideDebug true))

(fn `UserConstructionScript`
  ;[1 1 1] Makes Swap Enabled a switch that automatically toggles if this trigger is enabled or not. useful when copying-pasting triggers and need to quickly swap them both without having to move one first then the other.
  (if (`self.SwapEnabled`)
    (set `self.Enabling?` (not (`self.Enabling?`)))
    (set `self.SwapEnabled` false))
  (`BillboardComponent.SetSprite` (`self.Icon`) (select `bool` (`self.Enabling?`) :`false` "/Engine/EditorMaterials/Cascade/CASC_ModuleDisable.CASC_ModuleDisable" :`true` "/Engine/EditorMaterials/GreyCheck.GreyCheck" :!type "Texture2D Object Reference")))