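; LockedGate is a gate Blueprint whose Cube blocks the way while Locked and disappears when not.
; SetDoorUnlocked stores its input in Locked, then sets the Cube's collision and visibility to match, so a true value locks the gate despite the name.
; BeginPlay applies the initial Locked value, and SetActiveGeneral forwards its Active flag to the same event, so activating shows the solid gate.
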(event `self.ReceiveBeginPlay`
  (`self.SetDoorUnlocked` (`self.locked`)))

(event `SetDoorUnlocked`
  (params (Unlocked :type Boolean))
  (bind _output_get (set `self.locked` Unlocked))
  (`PrimitiveComponent.SetCollisionEnabled` (`self.Cube`) (select `bool` (not _output_get) :`false` "QueryAndPhysics" :`true` "NoCollision" :!type "ECollisionEnabled Enum"))
  (`SceneComponent.SetVisibility` (`self.Cube`) _output_get false))

(event `/Game/Blueprints/Mechanics/GeneralActivateInterface.SetActiveGeneral`
  (params (Active :type Boolean))
  (`self.SetDoorUnlocked` Active))

(fn `UserConstructionScript`)