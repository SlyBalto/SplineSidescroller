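; Player weapon component for the Splinescroller character that fires the current weapon, tracks ammo and switches weapons.
; The player passes its aim arrow each tick, and delay-gated repeaters spawn pistol bullets or SMG grenades that inherit the owner's spline position and facing.
; A per-enum info array holds ownership and ammo, feeding the HUD.
; Empty weapons trigger switching, which wraps through the enum using DoN loop guards to skip unavailable weapons.
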(event `ToggleFiring`
  (params (Firing :type Boolean) (ArrowToUse :type "ArrowComponent Object Reference"))
  ;[1 1 1] weapon functionality
  (if Firing
    (`self.Fireshot` ArrowToUse)))

(event `StopFiring`)

(event `Fireshot`
  (params (ArrowToUse :type "ArrowComponent Object Reference"))
  (bind _owningplayer (`self.OwningPlayer`))
  (bind (_reachedend _atfirstbox _distance _currentspline) (break `/Game/Blueprints/Mechanics/SplineInfo` (`/Game/Blueprints/Player/SplinescrollerCharacter.SplineInfo` _owningplayer)))
  ;[1 1 1] weapon functionality
  (set `self.ArrowAim` ArrowToUse)
  (switch `/Game/Blueprints/Player/PlayerWeapons` (`self.CurrentWeapon`)
    (:`NewEnumerator0`
      (`self.PistolWeapon` 2000.0 1.5))
    (:`NewEnumerator4`
      (`self.PistolWeapon` 4000.0 0.8 0.1 (0.0 0.0 -25.0))
      (`self.PistolWeapon` 4000.0 0.8 0.1 (0.0 0.0 25.0) 1.0 false))
    (:`NewEnumerator1`
      (`self.BasicRepeater` 0.2)
      (`self.UseAmmo`)
      (`|SpawnActorFromClass` "/Game/Blueprints/Attacks/PlayerGrenade.PlayerGrenade_C" (`self.QuickTransform`) "Undefined" "MultiplyWithRoot" null _currentspline (`/Game/Blueprints/Player/SplinescrollerCharacter.DirFacing` _owningplayer) _reachedend _atfirstbox _distance 200.0 2500.0 1.5 null))))

(event `StopWeaponFunctionality`)

(event `GetCurrentOwner`
  (bind _assplinescroller_character (cast `/Game/Blueprints/Player/SplinescrollerCharacter` (`self.GetOwner`)))
  (set `self.OwningPlayer` _assplinescroller_character))

(event `self.ReceiveBeginPlay`
  (bind _weaponinfo (`self.WeaponInfo`))
  (bind _weaponinfo_2 (`self.WeaponInfo`))
  (`self.GetCurrentOwner`)
  (`KismetArrayLibrary.Array_Resize` _weaponinfo_2 (enumcount `/Game/Blueprints/Player/PlayerWeapons`))
  ;[1 1 1] sets Pistol to have infinite ammo and to automatically have it
  (`KismetArrayLibrary.Array_Set` _weaponinfo_2 0 (make `/Game/Blueprints/Player/PlayerWeaponInfo` true 0 true))
  (`KismetSystemLibrary.PrintString` (`KismetStringLibrary.Concat_StrStr` "array for " (`KismetStringLibrary.Conv_IntToString` (`KismetArrayLibrary.Array_Length` _weaponinfo_2)) " weapons") true true (struct :`G` 0.66 :`B` 1.0 :`A` 1.0) 9.0)
  (if (`self.GiveAllWeapons`)
    (for (_array_element _array_index) (`self.WeaponInfo`)
      (bind _structout (setmembers `/Game/Blueprints/Player/PlayerWeaponInfo` :`StructRef` _array_element :`HasWeapon` true :`Infinite Ammo` true))
      (`KismetArrayLibrary.Array_Set` _weaponinfo _array_index _structout true)
      (bind (_hasweapon _ammo _infiniteammo) (break `/Game/Blueprints/Player/PlayerWeaponInfo` (`|GetArrayItem` _weaponinfo _array_index)))
      (`KismetSystemLibrary.PrintString` (`KismetStringLibrary.Concat_StrStr` (`|GetEnumeratorNameAsString` (cast `/Game/Blueprints/Player/PlayerWeapons` (`KismetMathLibrary.Conv_IntToByte` _array_index))) " available: " (`KismetStringLibrary.Conv_BoolToString` _hasweapon) " infinite ammo: " (`KismetStringLibrary.Conv_BoolToString` _infiniteammo)) true true (struct :`R` 1.0 :`B` 0.080507 :`A` 1.0) 8.0))))

(event `ForceOverride`
  (params (SetWeapon :type "/Game/Blueprints/Player/PlayerWeapons Enum" :default "NewEnumerator0"))
  (set `self.CurrentWeapon` SetWeapon)
  (`self.UpdateWeaponHUD Info` (`/Game/Blueprints/Player/SplinescrollerCharacter.PlayerHUD` (`self.OwningPlayer`)) :!label _label))

(event `UpdateWeaponHUD Info`
  (params (PlayerHUD :type "/Game/Blueprints/HUD/Player/PlayerHUD Object Reference"))
  (bind _currentweapon (`self.CurrentWeapon`))
  (bind (_output_hasweapon _output_ammo _output_infiniteammo) (break `/Game/Blueprints/Player/PlayerWeaponInfo` (`|GetArrayItem` (`self.WeaponInfo`) (`KismetMathLibrary.Conv_ByteToInt` _currentweapon))))
  (`/Game/Blueprints/HUD/Player/PlayerHUD.UpdateWeaponName` PlayerHUD _currentweapon)
  (`/Game/Blueprints/HUD/Player/PlayerHUD.UpdateShowAmmoCounter` PlayerHUD (not _output_infiniteammo))
  (`/Game/Blueprints/HUD/Player/PlayerHUD.UpdateAmmoCounter` PlayerHUD _output_ammo))

(event `SwitchWeapon`
  (params (Override :type Boolean) (`Add/Subract` :type Integer) (OverrideSet :type "/Game/Blueprints/Player/PlayerWeapons Enum" :default "NewEnumerator0") (`Reset Limiter` :type Boolean :default true))
  (bind _returnvalue (enumcount `/Game/Blueprints/Player/PlayerWeapons`))
  (bind _returnvalue_2 (+ (`KismetMathLibrary.Conv_ByteToInt` (`self.CurrentWeapon`)) `Add/Subract`))
  (bind _returnvalue_3 (select `bool` (< _returnvalue_2 0) :`false` (mod _returnvalue_2 _returnvalue) :`true` (- _returnvalue 1)))
  (bind _returnvalue_4 (cast `/Game/Blueprints/Player/PlayerWeapons` (`KismetMathLibrary.Conv_IntToByte` _returnvalue_3)))
  (bind _returnvalue_5 (cast `/Game/Blueprints/Player/PlayerWeapons` (`KismetMathLibrary.Conv_IntToByte` _returnvalue_3)))
  (if `Reset Limiter`
    (`|ExecutionSequence`
      (:`then_0`
        (goto _label_2 :!via `Reset`))
      (:`then_1`
        (`/Engine/EditorBlueprintResources/StandardMacros.Do N` (enumcount `/Game/Blueprints/Player/PlayerWeapons`) :!label _label_2 ; Prevent infinite loops by limiting N to\nhow many weapons exist for player
          (:`Exit`
            _)))))
  (if Override
    (if (`|EnumInequality` OverrideSet (`self.CurrentWeapon`))
      (`self.StopWeaponFunctionality`)
      (set `self.CurrentWeapon` OverrideSet)
      (goto _label))
    (elif (`self.CheckIfWeaponIsAvailable` (`|GetArrayItem` (`self.WeaponInfo`) _returnvalue_3))
      (`self.StopWeaponFunctionality`)
      (set `self.CurrentWeapon` _returnvalue_4)
      (goto _label)
      (else
        ;[1 1 1] prevents freezing from infinite loops
        (`|ExecutionSequence`
          (:`then_0`
            (goto _label_3 :!via `Reset`))
          (:`then_1`
            (`/Engine/EditorBlueprintResources/StandardMacros.Do N` (`KismetArrayLibrary.Array_Length` (`self.WeaponInfo`)) :!label _label_3
              (:`Exit`
                (`KismetSystemLibrary.PrintString` (`KismetStringLibrary.Concat_StrStr` (`|GetEnumeratorNameAsString` _returnvalue_4) " not available!"))
                (if (`self.CheckIfWeaponIsAvailable` (`|GetArrayItem` (`self.WeaponInfo`) _returnvalue_3))
                  (`self.ForceOverride` _returnvalue_5)
                  (else
                    (set `self.CurrentWeapon` _returnvalue_5)
                    (goto _label_3)))))))))))