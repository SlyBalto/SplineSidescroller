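; Weapon pickup item that grants its configured weapon type to the Splinescroller character.
; On pickup it checks the player's WeaponComp WeaponInfo array, indexed by the weapon enum.
; A new weapon is flagged as owned, debug-printed and force-switched to, then the item is removed.
; An already-owned weapon only removes the item; the ammo grant is noted in a comment but not implemented.
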(event `self.PickupItem`
  (params (SplinescrollerCharacter :type "/Game/Blueprints/Player/SplinescrollerCharacter Object Reference"))
  (bind _weaponcomp (`/Game/Blueprints/Player/SplinescrollerCharacter.WeaponComp` SplinescrollerCharacter))
  (bind _returnvalue (`KismetMathLibrary.Conv_ByteToInt` (`self.Weapon`)))
  (bind _weaponinfo (`/Game/Blueprints/Mechanics/WeaponComp.WeaponInfo` _weaponcomp))
  (bind _output (`|GetArrayItem` _weaponinfo _returnvalue))
  (bind _output_get (set `self.PlayerHasWeaponAlready` (`.HasWeapon_1_F0B70F1C4099BD3705C0FEBCAA71C779` (break `/Game/Blueprints/Player/PlayerWeaponInfo` _output))))
  (if _output_get
    ;[1 1 1] give ammo only
    (`self.RemoveItemFromGame`)
    (else
      (bind _structout (setmembers `/Game/Blueprints/Player/PlayerWeaponInfo` :`StructRef` _output :`HasWeapon` true))
      (`KismetArrayLibrary.Array_Set` _weaponinfo _returnvalue _structout)
      (`KismetSystemLibrary.PrintString` (`KismetStringLibrary.Concat_StrStr` "has " (`|GetEnumeratorNameAsString` (`self.Weapon`)) ": " (`KismetStringLibrary.Conv_BoolToString` (`.HasWeapon_1_F0B70F1C4099BD3705C0FEBCAA71C779` (break `/Game/Blueprints/Player/PlayerWeaponInfo` _output)))))
      (`/Game/Blueprints/Mechanics/WeaponComp.SwitchWeapon` _weaponcomp true 0 (`self.Weapon`) true)
      (`self.RemoveItemFromGame`))))

(fn `UserConstructionScript`
  (`parent.UserConstructionScript`))