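; Abstract base for pickup items in a spline-scroller game, with a spinning mesh and a Sphere trigger.
; Overlap by a SplinescrollerCharacter calls PickupItem, which by default destroys the actor through RemoveItemFromGame.
; Dropped items add a ProjectileMovement component at BeginPlay with an upward launch velocity.
; Otherwise, with SnapToFloor set, the construction script line-traces down to world-static geometry and places the item above it.
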(event `self.ReceiveBeginPlay`
  (`MovementComponent.SetUpdatedComponent` (`self.RotatingMovement`) (`self.ItemMesh`)) ; RotatingMovement components are normally\nfor the whole actor, but we just want the ItemMesh\nto be rotating.
  (if (`self.Dropped?`)
    (bind _returnvalue (`AddComponent|NODE_AddProjectileMovementComponent-0`))
    (set `MovementComponent.Velocity` (0.0 0.0 100.0) _returnvalue)))

(event `PickupItem`
  (params (SplinescrollerCharacter :type "/Game/Blueprints/Player/SplinescrollerCharacter Object Reference"))
  (`self.RemoveItemFromGame`))

(event `RemoveItemFromGame`
  (`self.K2_DestroyActor`))

(event `self.Sphere.OnComponentBeginOverlap`
  (params (OverlappedComponent :type "PrimitiveComponent Object Reference") (OtherActor :type "Actor Object Reference") (OtherComp :type "PrimitiveComponent Object Reference") (OtherBodyIndex :type Integer) (bFromSweep :type Boolean) (SweepResult :type "HitResult Structure (by ref)"))
  (bind _assplinescroller_character (cast `/Game/Blueprints/Player/SplinescrollerCharacter` OtherActor))
  (`self.PickupItem` _assplinescroller_character))

(fn `UserConstructionScript`
  (bind _returnvalue (`self.K2_GetActorLocation`))
  (if (and (`self.SnapToFloor`) (not (`self.Dropped?`)))
    (bind (_outhit _returnvalue_2) (`KismetSystemLibrary.LineTraceSingleForObjects` (+ _returnvalue (0.0 0.0 15.0)) (- _returnvalue (0.0 0.0 150.0)) (`|MakeArray` "ObjectTypeQuery1" :!type "EObjectTypeQuery Enum") true))
    (if _returnvalue_2
      (`self.K2_SetActorLocation` (+ (`.Location` (`GameplayStatics.BreakHitResult` _outhit)) (`KismetMathLibrary.MakeVector` 0.0 0.0 90.0))))))