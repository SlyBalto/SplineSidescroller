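; BasicEnemy is an enemy that fires homing bullets at the third-person character once it overlaps the trigger sphere.
; The overlap starts an endless delayed loop that spawns bullets aimed at the character's capsule, with no exit on leaving.
; A HealthSystem component tests overlaps on the sphere mesh and flashes it on damage.
; TookDamage also supports non-overlap damage sources and destroys the actor on death, while DamageSuccessful prints hits.
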(event `self.Spheretrigger.OnComponentBeginOverlap`
  (params (OverlappedComponent :type "PrimitiveComponent Object Reference") (OtherActor :type "Actor Object Reference") (OtherComp :type "PrimitiveComponent Object Reference") (OtherBodyIndex :type Integer) (bFromSweep :type Boolean) (SweepResult :type "HitResult Structure (by ref)"))
  (bind _returnvalue (`self.K2_GetActorLocation`))
  (bind _asbp_third_person_character (cast `/Game/Blueprints/Player/BP_ThirdPersonCharacter` OtherActor))
  (`|SpawnActorFromClass` "/Game/Blueprints/Attacks/BulletBasicHoming.BulletBasicHoming_C" (`KismetMathLibrary.MakeTransform` _returnvalue (`KismetMathLibrary.FindLookAtRotation` _returnvalue (`self.K2_GetActorLocation` _asbp_third_person_character)) (`KismetMathLibrary.Conv_DoubleToVector` 1.0)) "Undefined" "MultiplyWithRoot" null (`Character.CapsuleComponent` _asbp_third_person_character) self 500.0 3.0 null :!label _label)
  (`KismetSystemLibrary.Delay` 0.2)
  (goto _label))

(event `/Game/Blueprints/Mechanics/HealthAndDamageInterface.DamageSuccessful`
  (`KismetSystemLibrary.PrintString` (`KismetStringLibrary.Concat_StrStr` (`KismetSystemLibrary.GetDisplayName` self) " landed a hit!") true true (struct :`R` 1.0 :`G` 0.106714 :`B` 0.975415 :`A` 1.0) 6.0))

(event `self.SphereMesh.OnComponentBeginOverlap`
  (params (OverlappedComponent :type "PrimitiveComponent Object Reference") (OtherActor :type "Actor Object Reference") (OtherComp :type "PrimitiveComponent Object Reference") (OtherBodyIndex :type Integer) (bFromSweep :type Boolean) (SweepResult :type "HitResult Structure (by ref)"))
  (`/Game/Blueprints/Mechanics/HealthSystem.HealthOverlapTest` (`self.HealthSystem`) OtherComp))

(event `/Game/Blueprints/Mechanics/HealthAndDamageInterface.TookDamage`
  (params (Dead :type Boolean) (AttackingActor :type "Actor Object Reference") (`Health Left` :type Integer) (`Health Left Percent` :type "Float (double-precision)"))
  (if Dead
    (`self.K2_DestroyActor`)
    (else
      ;[1 1 1] Damage flashing only requires a ref of the mesh we want to flash. If there are multiple components, we can simply use the same nodes again.
      (`/Game/Blueprints/Mechanics/HealthSystem.DamageFlash` (`self.HealthSystem`) (`self.SphereMesh`)))))

(fn `UserConstructionScript`)