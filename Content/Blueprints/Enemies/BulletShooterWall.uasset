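; BulletShooterWall is an enemy hazard that fires repeated volleys of lightweight enemy bullets from a row of muzzles.
; The construction script creates evenly spaced, centered arrow components along local Y, with count and spacing set by variables.
; While active, SetActiveGeneral loops on FireDelay, using a DoN macro as a loop to spawn a bullet at every arrow.
; BeginPlay also runs a debug loop that continually prints the world's enemy bullet count.
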(event `FireBullet`
  (params (ArrowRef :type "SceneComponent Object Reference"))
  (`|SpawnActorFromClass` "/Game/Blueprints/Attacks/BulletLightweight_Enemy.BulletLightweight_Enemy_C" (`SceneComponent.K2_GetComponentToWorld` ArrowRef) "AlwaysSpawn" "MultiplyWithRoot" null (`self.BulletSpeed`) 6.0 null))

(event `/Game/Blueprints/Mechanics/GeneralActivateInterface.SetActiveGeneral`
  (params (Active :type Boolean))
  (bind _output_get (set `self.Active` Active))
  (if _output_get :!label _label
    (`|ExecutionSequence`
      (:`then_0`
        (goto _label_2 :!via `Reset`))
      (:`then_1`
        (bind _counter (`/Engine/EditorBlueprintResources/StandardMacros.Do N` (`self.Rows`) :!label _label_2)
          (:`Exit`
            (`self.FireBullet` (`|GetArrayItem` (`self.Arrows`) (- _counter 1)))
            (goto _label_2))))
      (:`then_2`
        (`KismetSystemLibrary.Delay` (`self.FireDelay`))
        (goto _label)))))

(event `self.ReceiveBeginPlay`
  (bind _outactors (`GameplayStatics.GetAllActorsOfClass` "/Game/Blueprints/Attacks/BulletLightweight_Enemy.BulletLightweight_Enemy_C" :!label _label_3))
  (`KismetSystemLibrary.PrintString` (`KismetStringLibrary.Concat_StrStr` (`KismetStringLibrary.Conv_IntToString` (`KismetArrayLibrary.Array_Length` _outactors)) " bullets in the world") true true (struct :`G` 0.66 :`B` 1.0 :`A` 1.0) 2.0 "bulebulelt count")
  (`KismetSystemLibrary.Delay` 0.1)
  (goto _label_3))

(fn `UserConstructionScript`
  (bind _returnvalue (`KismetMathLibrary.Conv_IntToDouble` (`self.Rows`)))
  (bind _returnvalue_2 (/ (* _returnvalue (`self.DistanceBetween`)) 2.0))
  (`KismetArrayLibrary.Array_Clear` (`self.Arrows`))
  (bind _counter (`/Engine/EditorBlueprintResources/StandardMacros.Do N` (`self.Rows`) :!label _label)
    (:`Exit`
      (bind _returnvalue_3 (`AddComponent|NODE_AddArrowComponent-0` :`RelativeTransform` (`KismetMathLibrary.MakeTransform` (`KismetMathLibrary.MakeVector` 0.0 (`KismetMathLibrary.MapRangeClamped` (`KismetMathLibrary.Conv_IntToDouble` _counter) 1.0 _returnvalue (* _returnvalue_2 -1.0) _returnvalue_2)) (struct :`Pitch` -90.0))))
      (`KismetArrayLibrary.Array_Add` (`self.Arrows`) _returnvalue_3)
      (goto _label))))