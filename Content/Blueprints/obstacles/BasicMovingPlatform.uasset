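; BasicMovingPlatform is an obstacle platform that moves from its starting position toward a marker component and removes bullets that hit it.
; On BeginPlay it caches its location and the world location of MoveTo1, then a Timeline alpha lerps the actor between them without sweeping.
; Hits on the Cube cast the other actor to BulletAbstract and call RemoveBulletFromGame on it.
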(event `self.ReceiveBeginPlay`
  (set `self.StartLoc` (`self.K2_GetActorLocation`))
  (set `self.GoToLoc` (`SceneComponent.K2_GetComponentLocation` (`self.MoveTo1`)))
  (bind (_direction _alpha) (`Timeline|Timeline`)
    (:`Update`
      (`self.K2_SetActorLocation` (`KismetMathLibrary.VLerp` (`self.StartLoc`) (`self.GoToLoc`) _alpha)))))

(event `self.Cube.OnComponentHit`
  (params (HitComponent :type "PrimitiveComponent Object Reference") (OtherActor :type "Actor Object Reference") (OtherComp :type "PrimitiveComponent Object Reference") (NormalImpulse :type "Vector Structure") (Hit :type "HitResult Structure (by ref)"))
  (bind _asbullet_abstract (cast `/Game/Blueprints/Attacks/BulletAbstract` OtherActor))
  (`/Game/Blueprints/Attacks/BulletAbstract.RemoveBulletFromGame` _asbullet_abstract))

(fn `UserConstructionScript`)